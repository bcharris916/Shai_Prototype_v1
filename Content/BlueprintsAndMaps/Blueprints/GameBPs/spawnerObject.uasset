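; Enemy spawner actor that creates an overworld enemy of its selected type (Slime, Warg, Magus or Goot) at its own transform.
; Shortly after BeginPlay it calls SpawnEnemy if active, which gives the new enemy a reference back to the spawner and clears IsActive.
; ActivateSpawner only sets the flag again, without spawning.
; A delayed random-chance spawn using RollChanceToSpawn exists but is disconnected.
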(event EventBeginPlay
  (Utilities|FlowControl|Delay 0.1)
  (if (Variables|Default|GetisActive)
    (CallFunction|SpawnEnemy)))

(event Collision|EventActorBeginOverlap
  (params (OtherActor :type Actor%20Object%20Reference)))

(event EventTick
  (params (DeltaSeconds :type Float%20%28single-precision%29)))

(fn ConstructionScript)

(fn SpawnEnemy
  (switch Utilities|FlowControl|Switch|SwitchonEnemyTypeEnum (Variables|Default|GetenemyType)
    (:NewEnumerator0
      (bind _returnvalue (Game|SpawnActorfromClass "/Game/BlueprintsAndMaps/Blueprints/EnemyBPs/Demo_BPs/overWorldEnemyPawnBP.overWorldEnemyPawnBP_C" (Transformation|GetActorTransform) "Undefined" 0 0 0))
      (bind _output_get (Variables|Default|SetspawnedEnemy _returnvalue))
      (Utilities|IsValid _output_get
        (:Is%20Valid
          (Variables|/Game/BlueprintsAndMaps/Blueprints/EnemyBPs/Demo_BPs/overWorldEnemyPawnBP.overWorldEnemyPawnBP_C|SetmySpawner _output_get self))
        (:Is%20Not%20Valid
          _)))
    (:NewEnumerator1
      (bind _returnvalue_2 (Game|SpawnActorfromClass "/Game/BlueprintsAndMaps/Blueprints/EnemyBPs/Demo_BPs/warg_enemyBP.warg_enemyBP_C" (Transformation|GetActorTransform) "Undefined" 0 0 0))
      (bind _output_get_2 (Variables|Default|SetspawnedEnemy _returnvalue_2))
      (Utilities|IsValid _output_get_2
        (:Is%20Valid
          (Variables|/Game/BlueprintsAndMaps/Blueprints/EnemyBPs/Demo_BPs/overWorldEnemyPawnBP.overWorldEnemyPawnBP_C|SetmySpawner _output_get_2 self))
        (:Is%20Not%20Valid
          _)))
    (:NewEnumerator2
      (bind _returnvalue_3 (Game|SpawnActorfromClass "/Game/BlueprintsAndMaps/Blueprints/EnemyBPs/Demo_BPs/magus_enemyBP.magus_enemyBP_C" (Transformation|GetActorTransform) "Undefined" 0 0 0))
      (bind _output_get_3 (Variables|Default|SetspawnedEnemy _returnvalue_3))
      (Utilities|IsValid _output_get_3
        (:Is%20Valid
          (Variables|/Game/BlueprintsAndMaps/Blueprints/EnemyBPs/Demo_BPs/overWorldEnemyPawnBP.overWorldEnemyPawnBP_C|SetmySpawner _output_get_3 self))
        (:Is%20Not%20Valid
          _)))
    (:NewEnumerator3
      (bind _returnvalue_4 (Game|SpawnActorfromClass "/Game/BlueprintsAndMaps/Blueprints/EnemyBPs/Demo_BPs/goot_enemyBP.goot_enemyBP_C" (Transformation|GetActorTransform) "Undefined" 0 0 0))
      (bind _output_get_4 (Variables|Default|SetspawnedEnemy _returnvalue_4))
      (Utilities|IsValid _output_get_4
        (:Is%20Valid
          (Variables|/Game/BlueprintsAndMaps/Blueprints/EnemyBPs/Demo_BPs/overWorldEnemyPawnBP.overWorldEnemyPawnBP_C|SetmySpawner _output_get_4 self))
        (:Is%20Not%20Valid
          _))))
  (Variables|Default|SetisActive false)
  (return))

(fn ActivateSpawner
  (Variables|Default|SetisActive true))

(fn RollChancetoSpawn
  (return (<= (Math|Random|RandomFloatinRange 0.0 (Variables|Default|GetchanceConstant)) (Variables|Default|GetchanceToSpawn))))