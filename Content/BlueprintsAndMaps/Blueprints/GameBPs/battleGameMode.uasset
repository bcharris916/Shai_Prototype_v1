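; Game mode for turn-based battles that creates the battle UI, alternates player and enemy turns, and routes damage.
; Turns pass via a flag on the battle controller and TakeTurn calls on every enemy pawn, with capped player energy regained after each player turn.
; Damage hits all enemies or the player and triggers flinching.
; An end-battle screen event resets player energy, stored through the main game instance.
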(event Custom|applyDamage
  (params (didPlayerDealDamage :type Boolean) (damageAmount :type Integer))
  ;[1 1 1] Apply Damage and call respective Pawns take damage events with an input boolean.
  (if didPlayerDealDamage
    (bind _outactors (Actor|GetAllActorsOfClass "/Game/BlueprintsAndMaps/Blueprints/EnemyBPs/Demo_BPs/overWorldEnemyPawnBP.overWorldEnemyPawnBP_C"))
    (for _array_element _outactors
      (Default|TakeDamage _array_element damageAmount)
      (Variables|/Game/BlueprintsAndMaps/Blueprints/EnemyBPs/Demo_BPs/overWorldEnemyPawnBP.overWorldEnemyPawnBP_C|SetisFlinching _array_element true))
    (else
      (bind _asbattle_player_bp (Utilities|Casting|CastTobattlePlayerBP (Game|GetPlayerCharacter 0)))
      (Default|TakeDamage _asbattle_player_bp damageAmount)
      (Variables|/Game/BlueprintsAndMaps/Blueprints/PlayerBPs/battlePlayerBP.battlePlayerBP_C|SetisFlinching _asbattle_player_bp true))))

(event Custom|displayEndBattleScreen
  ;[1 1 1] Display End Battle Screen if a Player or Enemy is Defeated. Currently called when the Main Game Instance runs Event Change Mob Count. Although both of these thing should happen at end of battle, that is not where this should be called from.
  (bind _returnvalue (UserInterface|CreateWidget "/Game/BlueprintsAndMaps/Blueprints/UI_BPs/DemoBPs/endBattleScreen.endBattleScreen_C" (Game|GetPlayerController 0)))
  (Variables|Default|SetcurrentEndBattleScreen _returnvalue)
  (UserInterface|Viewport|AddtoViewport (Variables|Default|GetcurrentEndBattleScreen) 0)
  (Variables|/Game/BlueprintsAndMaps/Blueprints/PlayerBPs/playerObjectBP.playerObjectBP_C|SetREFPlayerCurrentEnergy (Variables|/Game/BlueprintsAndMaps/Blueprints/GameBPs/mainGameInstance.mainGameInstance_C|GetMainGameInstancePlayerObjectBP (Variables|Default|GetmainGameInstanceREF)) 10))

(event Custom|startBattle
  ;[1 1 1] Starts and controls Player and Enemy Turns. This is curently kicked off and called from Battle Level BP.
  (CallFunction|PlayerTurn))

(event Custom|PlayerTurn
  ;[1 1 1] Starts and controls Player and Enemy Turns. This is curently kicked off and called from Battle Level BP.
  (Variables|/Game/BlueprintsAndMaps/Blueprints/PlayerBPs/battleControllerBP.battleControllerBP_C|SetplayerTurn (.AsBattle%20Controller%20BP (Utilities|Casting|CastTobattleControllerBP (Game|GetPlayerController 0))) true))

(event Custom|EnemyTurn
  ;[1 1 1] Starts and controls Player and Enemy Turns. This is curently kicked off and called from Battle Level BP.
  (bind _outactors (Actor|GetAllActorsOfClass "/Game/BlueprintsAndMaps/Blueprints/EnemyBPs/Demo_BPs/overWorldEnemyPawnBP.overWorldEnemyPawnBP_C"))
  (for _array_element _outactors
    (Default|TakeTurn _array_element)))

(event Custom|PlayerFinishedTurn
  (bind _maingameinstanceref (Variables|Default|GetmainGameInstanceREF))
  (bind _maingameinstanceplayerobjectbp (Variables|/Game/BlueprintsAndMaps/Blueprints/GameBPs/mainGameInstance.mainGameInstance_C|GetMainGameInstancePlayerObjectBP _maingameinstanceref))
  ;[1 1 1] Starts and controls Player and Enemy Turns. This is curently kicked off and called from Battle Level BP.
  (Variables|/Game/BlueprintsAndMaps/Blueprints/PlayerBPs/battleControllerBP.battleControllerBP_C|SetplayerTurn (.AsBattle%20Controller%20BP (Utilities|Casting|CastTobattleControllerBP (Game|GetPlayerController 0))) false)
  (if (> (+ (Variables|/Game/BlueprintsAndMaps/Blueprints/PlayerBPs/playerObjectBP.playerObjectBP_C|GetREFPlayerCurrentEnergy _maingameinstanceplayerobjectbp) 2) 10)
    (Variables|/Game/BlueprintsAndMaps/Blueprints/PlayerBPs/playerObjectBP.playerObjectBP_C|SetREFPlayerCurrentEnergy _maingameinstanceplayerobjectbp 10)
    (else
      (Variables|/Game/BlueprintsAndMaps/Blueprints/PlayerBPs/playerObjectBP.playerObjectBP_C|SetREFPlayerCurrentEnergy _maingameinstanceplayerobjectbp (+ (Variables|/Game/BlueprintsAndMaps/Blueprints/PlayerBPs/playerObjectBP.playerObjectBP_C|GetREFPlayerCurrentEnergy _maingameinstanceplayerobjectbp) 2))))
  (CallFunction|EnemyTurn))

(event Custom|enemyFinishedTurn
  ;[1 1 1] Starts and controls Player and Enemy Turns. This is curently kicked off and called from Battle Level BP.
  (CallFunction|PlayerTurn))

(event EventBeginPlay
  ;[1 1 1] On Begin Play Create and set/Add the Battle UI to viewport
  (bind _asbattle_controller_bp (Utilities|Casting|CastTobattleControllerBP (Game|GetPlayerController 0)))
  (bind _returnvalue (UserInterface|CreateWidget "/Game/BlueprintsAndMaps/Blueprints/UI_BPs/BattleUI.BattleUI_C" _asbattle_controller_bp))
  (Variables|Default|SetcurrentBattleUIInstance _returnvalue)
  (UserInterface|Viewport|AddtoViewport (Variables|Default|GetcurrentBattleUIInstance) 0)
  (bind _asmain_game_instance (Utilities|Casting|CastTomainGameInstance (Game|GetGameInstance)))
  (Variables|Default|SetmainGameInstanceREF _asmain_game_instance))

(fn ConstructionScript)