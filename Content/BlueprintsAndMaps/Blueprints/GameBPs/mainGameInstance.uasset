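; Game instance for an RPG that carries player, enemy and music state between overworld maps and battle levels.
; It constructs the player object for new or loaded games, saves it to a slot, and spawns enemies from data tables.
; The battled enemy's data is stored to drive damage, EXP and table-based level-ups.
; On level entry it picks the theme by map name and deactivates the last fought enemy's spawner.
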(event Custom|QuitAndSaveGame
  (params (quit? :type Boolean))
  ;[1 1 1] Quit and Save game from Overworld UI. Setting variables to Player Save Struct
  (if quit?
    (Game|QuitGame (Game|GetPlayerController 0) "Quit" false)
    (else
      (Default|UpdatePlayerStatsStructurefromREF (Variables|Default|GetMainGameInstancePlayerObjectBP))
      (bind _returnvalue (SaveGame|CreateSaveGameObject "/Game/BlueprintsAndMaps/Blueprints/GameBPs/PlayerSaveGameObject.PlayerSaveGameObject_C"))
      (bind _output_get (Variables|Default|SetcurrentPlayerSaveGameObject _returnvalue))
      (Variables|/Game/BlueprintsAndMaps/Blueprints/GameBPs/PlayerSaveGameObject.PlayerSaveGameObject_C|SetquestEvents _output_get (Variables|Default|GetREFplayerQuestEvents))
      (Variables|/Game/BlueprintsAndMaps/Blueprints/GameBPs/PlayerSaveGameObject.PlayerSaveGameObject_C|SetREFPlayerStatsStructure _output_get (Variables|/Game/BlueprintsAndMaps/Blueprints/PlayerBPs/playerObjectBP.playerObjectBP_C|GetplayerStatsStructure (Variables|Default|GetMainGameInstancePlayerObjectBP)))
      (bind _returnedplayersaveslot (Default|ReturnPlayerSaveSlot (Variables|Default|GetMainGameInstancePlayerObjectBP)))
      (SaveGame|SaveGametoSlot (Variables|Default|GetcurrentPlayerSaveGameObject) _returnedplayersaveslot))))

(event Custom|updatePlayerOnLoad
  (params (loadedPlayerSaveObject :type Player%20Stats%20Structure%20Structure))
  (bind (_playercurrenthealth _playermaxhealth _playerexp _playerexptonextlevel _playerlevel _playerbasepower _profilename _playersaveslot _previousplayerexptonextlevel _currentlevelname _playerallweapons _playerallskills _playerequippedskills) (Utilities|Struct|BreakPlayerStatsStructure loadedPlayerSaveObject))
  (bind _maingameinstanceplayerobjectbp (Variables|Default|GetMainGameInstancePlayerObjectBP))
  (bind _maingameinstanceplayerobjectbp_2 (Variables|Default|GetMainGameInstancePlayerObjectBP))
  ;[1 1 1] Updates Player on Load of Game from save Game Object. Updates our current Structure of the Player
  (CallFunction|ConstructPlayerObject)
  (Default|UpdatePlayerStatsStructurefromSaveGameObject (Variables|Default|GetMainGameInstancePlayerObjectBP) loadedPlayerSaveObject)
  (Default|LoadInventory _maingameinstanceplayerobjectbp_2 _playerallweapons)
  (Default|AddSkilltoAllSkillsbySkillData _maingameinstanceplayerobjectbp_2 _playerallskills)
  (Default|AddSkilltoEquippedbyData _maingameinstanceplayerobjectbp _playerequippedskills)
  (Default|SetTotalPower _maingameinstanceplayerobjectbp))

(event Custom|loadEnemiesByLevel
  (params (levelName :type Name))
  ;[1 1 1] Prototype Enemy Spawn by level name event. We will call this on New Game/Load Game and map change. Two Modes: Dev Mode doesnt spawn by level type, and Normal mode which does spawn by level type.
  (CallFunction|SetLoadedEnemiesArraybyLevel levelName)
  (CallFunction|SpawnLoadedEnemies))

(event Custom|playerEnteredLevel
  ;[1 1 1] Prototype Enemy Spawn by level name event. We will call this on New Game/Load Game and map change. Two Modes: Dev Mode doesnt spawn by level type, and Normal mode which does spawn by level type.
  (bind _returnvalue (Game|GetCurrentLevelName true))
  (if (Utilities|Enum|Equal(Enum) (Variables|Default|GetvillageMapName) _returnvalue)
    (if (Variables|Default|GetisVillageTheme)
      _
      (else
        (CallFunction|PlayVIllageTheme)))
    (else
      (bind _returnvalue_2 (Game|GetCurrentLevelName true))
      (if (Utilities|Enum|Equal(Enum) (Variables|Default|GetspecialThemeMap) _returnvalue_2)
        (if (Variables|Default|GetisVIllainTheme)
          _
          (else
            (CallFunction|PlayVillainTheme)))
        (elif (Variables|Default|GetisFieldTheme)
          _
          (else
            (CallFunction|PlayFieldTheme))))))
  (bind _outactors (Actor|GetAllActorsOfClass "/Game/BlueprintsAndMaps/Blueprints/GameBPs/spawnerObject.spawnerObject_C"))
  (bind _array_element (Utilities|Array|ForEachLoopwithBreak _outactors)
    (:LoopBody
      (if (== (Variables|/Game/BlueprintsAndMaps/Blueprints/GameBPs/spawnerObject.spawnerObject_C|GetspawnerIndex _array_element) (Variables|Default|GetspawnerToDeactivate))
        (Variables|/Game/BlueprintsAndMaps/Blueprints/GameBPs/spawnerObject.spawnerObject_C|SetisActive _array_element false)))))

(event Custom|calculateDamageCurrentBattleEnemyBySkillIndex
  (params (skillIndex :type Integer))
  (bind _currentbattleenemyoverworlddata (Variables|Default|GetcurrentBattleEnemyOverworldData))
  ;[1 1 1] Updated Enemy Damage System for Battle
  (Default|UpdateEnemyPower _currentbattleenemyoverworlddata)
  (bind _damagebyskill (Default|CalcDamagebySkillIndex _currentbattleenemyoverworlddata skillIndex))
  (bind _asbattle_game_mode (Utilities|Casting|CastTobattleGameMode (Game|GetGameMode)))
  (Default|ApplyDamage _asbattle_game_mode false _damagebyskill))

(event Custom|loadEnemyByName
  (params (enemyName :type Name))
  (bind (_activemobspawndata _addedenemypawn) (CallFunction|SpawnSingleEnemyatDefaultLocation enemyName))
  (bind _returnvalue (Utilities|Array|Add (Variables|Default|GetactiveMobSpawns) _activemobspawndata))
  (Variables|/Game/BlueprintsAndMaps/Blueprints/EnemyBPs/Demo_BPs/overWorldEnemyPawnBP.overWorldEnemyPawnBP_C|SetcurrentEnemyIndex _addedenemypawn _returnvalue))

(event Custom|playVIllageTheme
  (if (not (Variables|Default|GetmusicDisabled?))
    (Utilities|IsValid (Variables|Default|GetmyCurrentTheme)
      (:Is%20Valid
        (Audio|Components|Audio|Stop (Variables|Default|GetmyCurrentTheme)))
      (:Is%20Not%20Valid
        _))
    (bind _returnvalue (Audio|SpawnSound2D "/Game/Audio/sound_Village_Theme.sound_Village_Theme" 1.0 1.0 0.0 0 true false))
    (Variables|Default|SetmyCurrentTheme _returnvalue)
    (Variables|Default|SetisFieldTheme false)
    (Variables|Default|SetisVillageTheme true)))

(event Custom|playVillainTheme
  (if (not (Variables|Default|GetmusicDisabled?))
    (Utilities|IsValid (Variables|Default|GetmyCurrentTheme)
      (:Is%20Valid
        (Audio|Components|Audio|Stop (Variables|Default|GetmyCurrentTheme)))
      (:Is%20Not%20Valid
        _))
    (bind _returnvalue (Audio|SpawnSound2D "/Game/Audio/Shai_VIllain_Theme.Shai_VIllain_Theme" 1.0 1.0 0.0 0 true false))
    (Variables|Default|SetmyCurrentTheme _returnvalue)
    (Variables|Default|SetisFieldTheme false)
    (Variables|Default|SetisVillageTheme false)
    (Variables|Default|SetisVIllainTheme true)))

(event Custom|playMenuTheme
  (if (not (Variables|Default|GetmusicDisabled?))
    (Utilities|IsValid (Variables|Default|GetmyCurrentTheme)
      (:Is%20Valid
        (Audio|Components|Audio|Stop (Variables|Default|GetmyCurrentTheme)))
      (:Is%20Not%20Valid
        _))
    (bind _returnvalue (Audio|SpawnSound2D "/Game/Audio/sound_Hero_theme.sound_Hero_theme" 1.0 1.0 0.0 0 false false))
    (Variables|Default|SetmyCurrentTheme _returnvalue)
    (Variables|Default|SetisFieldTheme false)
    (Variables|Default|SetmenuThemePlaying true)))

(event Custom|playFieldTheme
  (if (not (Variables|Default|GetmusicDisabled?))
    (if (not (Variables|Default|GetisFieldTheme))
      (Utilities|IsValid (Variables|Default|GetmyCurrentTheme)
        (:Is%20Valid
          (Audio|Components|Audio|Stop (Variables|Default|GetmyCurrentTheme)))
        (:Is%20Not%20Valid
          _))
      (bind _returnvalue (Audio|SpawnSound2D "/Game/Audio/Shai_Battle_theme.Shai_Battle_theme" 1.0 1.0 0.0 0 true false))
      (Variables|Default|SetmyCurrentTheme _returnvalue)
      (Variables|Default|SetisFieldTheme true)
      (Variables|Default|SetisVillageTheme false)
      (Variables|Default|SetisVIllainTheme false))))

(event Custom|playBattleTheme
  (if (not (Variables|Default|GetmusicDisabled?))
    (Audio|Components|Audio|Stop (Variables|Default|GetmyCurrentTheme))
    (bind _returnvalue (Audio|SpawnSound2D "/Game/Audio/Shai_Battle_theme.Shai_Battle_theme" 1.0 1.0 0.0 0))
    (Variables|Default|SetmyCurrentTheme _returnvalue)
    (Variables|Default|SetisFieldTheme false)
    (Variables|Default|SetmenuThemePlaying false)))

(event Custom|setPlayerToReviveState
  (bind _maingameinstanceplayerobjectbp (Variables|Default|GetMainGameInstancePlayerObjectBP))
  (Viewport|RemoveAllWidgets)
  (bind _returnvalue (UserInterface|CreateWidget "/Game/BlueprintsAndMaps/Blueprints/UI_BPs/reviveUI.reviveUI_C" (Game|GetPlayerController 0)))
  (UserInterface|Viewport|AddtoViewport _returnvalue 0)
  (Variables|/Game/BlueprintsAndMaps/Blueprints/PlayerBPs/playerObjectBP.playerObjectBP_C|SetREFPlayerCurrentHealth _maingameinstanceplayerobjectbp (Variables|/Game/BlueprintsAndMaps/Blueprints/PlayerBPs/playerObjectBP.playerObjectBP_C|GetREFPlayerMaxHealth _maingameinstanceplayerobjectbp)))

(event Custom|changeMobSpawnCount
  (params (activeMobNum :type Integer) (defeateEnemyData :type Enemy%20Data%20Structure%20Structure) (enemyIndex :type Integer))
  ;[1 1 1] Game Instance wants to keep track of how many Mobs should currently be spawning on this tile.
  (Utilities|Array|RemoveIndex (Variables|Default|GetactiveMobSpawns) enemyIndex)
  (Variables|Default|SetcurrentMobCount (- (Variables|Default|GetcurrentMobCount) activeMobNum))
  (bind _asbattle_game_mode (Utilities|Casting|CastTobattleGameMode (Game|GetGameMode)))
  (Default|DisplayEndBattleScreen _asbattle_game_mode))

(event Custom|playStartBattleSound
  (bind _returnvalue (Audio|SpawnSound2D "/Game/Audio/soundBattleStart.soundBattleStart" 1.0 1.0 0.0 0 true))
  (Audio|Components|Audio|Play _returnvalue 0.0))

(event Custom|revivePlayer
  (bind _currentbattleenemyoverworlddata (Variables|Default|GetcurrentBattleEnemyOverworldData))
  (CallFunction|UpdatePlayerAfterBattle)
  (Utilities|IsValid _currentbattleenemyoverworlddata
    (:Is%20Valid
      (Actor|DestroyActor _currentbattleenemyoverworlddata))
    (:Is%20Not%20Valid
      _))
  (Variables|Default|SetisBattle? false)
  (Game|OpenLevel(byName) (Utilities|String|StringToName (Variables|Default|GetvillageMapName))))

(event Custom|setBattleEnemyType
  (params (overWorldPawnEnemyREF :type Over%20World%20Enemy%20Pawn%20BP%20Object%20Reference))
  (bind _myspawner (Variables|/Game/BlueprintsAndMaps/Blueprints/EnemyBPs/Demo_BPs/overWorldEnemyPawnBP.overWorldEnemyPawnBP_C|GetmySpawner overWorldPawnEnemyREF))
  ;[1 1 1] Game Instance can Set the Enemy Battle type so that the Battle Game Mode will know what Enemy is battling. Storing some reward information ehre like Exp for now since it is a great time to get this data off the enemy while the referenc is valid.
  (Utilities|IsValid _myspawner
    (:Is%20Valid
      (Variables|Default|SetspawnerToDeactivate (Variables|/Game/BlueprintsAndMaps/Blueprints/GameBPs/spawnerObject.spawnerObject_C|GetspawnerIndex _myspawner)))
    (:Is%20Not%20Valid
      _))
  (Variables|Default|SetREF_BattleEnemyType (Utilities|GetClass overWorldPawnEnemyREF))
  (bind _output_get (Variables|Default|SetcurrentBattleEnemyOverworldData overWorldPawnEnemyREF))
  (bind _returnvalue (Game|ConstructObjectfromClass "/Game/BlueprintsAndMaps/Blueprints/EnemyBPs/enemyObject_BP.enemyObject_BP_C" self))
  (bind _output_get_2 (Variables|Default|SetcurrentBattleEnemyObject _returnvalue))
  (Variables|/Game/BlueprintsAndMaps/Blueprints/EnemyBPs/enemyObject_BP.enemyObject_BP_C|SetenemyDataStructure _output_get_2 (Variables|/Game/BlueprintsAndMaps/Blueprints/EnemyBPs/enemyObject_BP.enemyObject_BP_C|GetenemyDataStructure (Variables|/Game/BlueprintsAndMaps/Blueprints/EnemyBPs/Demo_BPs/overWorldEnemyPawnBP.overWorldEnemyPawnBP_C|GetenemyObject _output_get))))

(event Custom|UpdatePlayerAfterBattle
  (bind _maingameinstanceplayerobjectbp (Variables|Default|GetMainGameInstancePlayerObjectBP))
  ;[1 1 1] Current Update we call at end of Battle. Checks if we flee'd and if not gives us our loot and or levels us up.
  (CallFunction|SetEnemyLoot)
  (Variables|Default|SetTempPlayerCurrentExp (+ (Utilities|Array|Get(acopy) (Variables|Default|GetcurrentEnemyExpOnDefeat) 1) (Variables|/Game/BlueprintsAndMaps/Blueprints/PlayerBPs/playerObjectBP.playerObjectBP_C|GetREFPlayerCurrentExp _maingameinstanceplayerobjectbp)))
  (if (>= (Variables|Default|GetTempPlayerCurrentExp) (Variables|/Game/BlueprintsAndMaps/Blueprints/PlayerBPs/playerObjectBP.playerObjectBP_C|GetREFPlayerExpToNextLevel _maingameinstanceplayerobjectbp))
    (CallFunction|LevelUpPlayer)
    (else
      (Variables|/Game/BlueprintsAndMaps/Blueprints/PlayerBPs/playerObjectBP.playerObjectBP_C|SetREFPlayerCurrentExp (Variables|Default|GetMainGameInstancePlayerObjectBP) (Variables|Default|GetTempPlayerCurrentExp))))
  (Default|UpdatePlayerStatsStructurefromREF (Variables|Default|GetMainGameInstancePlayerObjectBP)))

(event Custom|endBattle
  (bind _currentbattleenemyoverworlddata (Variables|Default|GetcurrentBattleEnemyOverworldData))
  ;[1 1 1] Game Instance is Ending Battle and Opening Overworld Map. Opening the next level should definately be on Battle Game Mode and may be redundant here. Prototype Level Up system for Save Game Prototype here currently.
  (if (Variables|Default|GetplayerFlee?)
    (CallFunction|DestroyPlayerLocators)
    (Variables|Default|SetplayerFlee? false)
    (Variables|Default|SetisBattle? false :!label _label)
    (Game|OpenLevel(byName) (Variables|Default|GetplayerMapNameBeforeBattle))
    (Variables|Default|SetendedBattleScene true)
    (bind _returnvalue (Audio|SpawnSound2D "/Game/Audio/UISounds/sound_magical_whoosh.sound_magical_whoosh" 1.0 1.0 0.0 0 true))
    (Audio|Components|Audio|Play _returnvalue 0.0)
    (else
      (CallFunction|UpdatePlayerAfterBattle)
      (if (Variables|Default|GetisBattle?)
        (goto _label)
        (else
          (Utilities|IsValid _currentbattleenemyoverworlddata
            (:Is%20Valid
              (Actor|DestroyActor _currentbattleenemyoverworlddata)
              (CallFunction|DestroyPlayerLocators))))))))

(event Custom|levelUpPlayer
  (bind _maingameinstanceplayerobjectbp (Variables|Default|GetMainGameInstancePlayerObjectBP))
  (bind _refplayerlevel (Variables|/Game/BlueprintsAndMaps/Blueprints/PlayerBPs/playerObjectBP.playerObjectBP_C|GetREFPlayerLevel _maingameinstanceplayerobjectbp))
  ;[1 1 1] Calls two fn.'s that add to player Max HP and set the Exp to Next Level. Weird shit in the fns. check google sheets.
  (if (<= _refplayerlevel (Variables|Default|GetplayerLevelCap))
    (Math|Integer|IncrementInt _refplayerlevel
      (:%20%20
        (CallFunction|SetMaxHponLevel)
        (CallFunction|SetExptoNextLevel)
        (Default|SetTotalPower _maingameinstanceplayerobjectbp)
        (Default|UpdatePlayerStatsStructurefromREF (Variables|Default|GetMainGameInstancePlayerObjectBP))))))

(event Custom|openInventoryUI
  ;[1 1 1] Prototype For Inventory UI..integrates Instantiating an Inventory Object on the player at the game intances call, ref the game isntance player object on the inventory UI to get all weapons and display them.
  (bind _returnvalue (UserInterface|CreateWidget "/Game/BlueprintsAndMaps/Blueprints/UI_BPs/PlayerWeaponSkillsUI.PlayerWeaponSkillsUI_C"))
  (UserInterface|Viewport|AddtoViewport _returnvalue 0))

(event Custom|updatePlayerNewGame
  (bind _maingameinstanceplayerobjectbp (Variables|Default|GetMainGameInstancePlayerObjectBP))
  (bind _starterskills (Variables|/Game/BlueprintsAndMaps/Blueprints/PlayerBPs/playerObjectBP.playerObjectBP_C|GetStarterSkills _maingameinstanceplayerobjectbp))
  ;[1 1 1] Player Initialization code goes here for now.
  (CallFunction|ConstructPlayerObject)
  (Default|UpdateREFVariablesfromPlayerStatsStructure (Variables|Default|GetMainGameInstancePlayerObjectBP))
  ;;[1 1 1] Gives our player testable weapons and skills on new game.
  (Default|PlayerAquiresWeapon (Variables|Default|GetMainGameInstancePlayerObjectBP) "WoodStick")
  (Default|PlayerAquiresSkill _maingameinstanceplayerobjectbp _starterskills)
  (Default|AddSkilltoEquippedbyName (Variables|Default|GetMainGameInstancePlayerObjectBP) _starterskills)
  (Variables|/Game/BlueprintsAndMaps/Blueprints/PlayerBPs/playerObjectBP.playerObjectBP_C|SetREFProfileName (Variables|Default|GetMainGameInstancePlayerObjectBP) (Variables|Default|GetProfileName))
  (Variables|/Game/BlueprintsAndMaps/Blueprints/PlayerBPs/playerObjectBP.playerObjectBP_C|SetREFPlayerSaveSlot (Variables|Default|GetMainGameInstancePlayerObjectBP) (Variables|Default|GetPlayerSaveSlot))
  (Default|UpdatePlayerStatsStructurefromREF (Variables|Default|GetMainGameInstancePlayerObjectBP)))

(event Custom|constructPlayerObject
  ;[1 1 1] Creates an Instance of PlayerObject for use on Load or New Game
  (bind _returnvalue (Game|ConstructObjectfromClass "/Game/BlueprintsAndMaps/Blueprints/PlayerBPs/playerObjectBP.playerObjectBP_C" self))
  (Variables|Default|SetMainGameInstancePlayerObjectBP _returnvalue))

(fn CalcBonusHPonLevel
  (params (playerLevel :type Integer))
  (LocalVariables|SetplayerLevelREF playerLevel)
  (bind _output_get (LocalVariables|SettotalBonusHP (Math|Float|Truncate (* (* (LocalVariables|GetplayerLevelREF) (LocalVariables|GetHealthPiValue)) (* (LocalVariables|GetplayerLevelREF) (LocalVariables|GetHealthGoldenRatio))))))
  (return _output_get))

(fn CalcExptoNextLevel
  (params (PlayerLevel :type Integer))
  ;[1 1 1] Check google sheets player scaling for explanation of this weird shit.
  (LocalVariables|SetplayerLevelREF PlayerLevel)
  (LocalVariables|SetpumpUpValue (* (LocalVariables|GetplayerLevelREF) (LocalVariables|GetbaseValue)))
  (LocalVariables|SetAddedVariationValue (* (Math|Float|Power (Math|Conversions|ToFloat(Integer) (LocalVariables|GetplayerLevelREF)) 1.6) 1e+02))
  (LocalVariables|SetLevelMultiplierValue (Math|Float|Power 1.6 (Math|Conversions|ToFloat(Integer) (LocalVariables|GetplayerLevelREF))))
  (return (+ (Math|Float|Floor (LocalVariables|GetAddedVariationValue)) (Math|Float|Truncate (* (LocalVariables|GetLevelMultiplierValue) (LocalVariables|GetpumpUpValue))))))

(fn SetLoadedEnemiesArraybyLevel
  (params (levelByName :type Name))
  (bind _returnvalue (Utilities|GetDataTableRow "/Game/BlueprintsAndMaps/Blueprints/GameBPs/LevelBPs/LevelDataTable.LevelDataTable" levelByName)
    (:then
      (for _array_element (.enemiesToSpawnByName (Utilities|Struct|BreakLevelDataStructure _returnvalue))
        (Utilities|Array|Add (Variables|Default|GetLoadedEnemiesByName) _array_element)
        (return)))))

(fn SpawnLoadedEnemies
  (bind _overworldenemyorigin (Variables|Default|GetoverworldEnemyOrigin))
  (for (_array_element _array_index) (Variables|Default|GetLoadedEnemiesByName)
    (bind _returnvalue (Utilities|GetDataTableRow "/Game/BlueprintsAndMaps/Blueprints/EnemyBPs/EnemyDataTable.EnemyDataTable" _array_element)
      (:then
        (bind _returnvalue_2 (Game|SpawnActorfromClass (.enemyClass (Utilities|Struct|BreakEnemyDataStructure _returnvalue)) (Math|Transform|MakeTransform (Math|Vector|MakeVector (+ (.x _overworldenemyorigin) (Math|Random|RandomFloatinRange -5e+02 5e+02)) (+ (.y _overworldenemyorigin) (Math|Random|RandomFloatinRange -5e+02 5e+02)) (.z _overworldenemyorigin)) "0,180.000000, 0") "AdjustIfPossibleButAlwaysSpawn" 0 _array_index 0))
        (bind _returnvalue_3 (Game|ConstructObjectfromClass "/Game/BlueprintsAndMaps/Blueprints/EnemyBPs/enemyObject_BP.enemyObject_BP_C" _returnvalue_2))
        (bind _output_get (Variables|/Game/BlueprintsAndMaps/Blueprints/EnemyBPs/Demo_BPs/overWorldEnemyPawnBP.overWorldEnemyPawnBP_C|SetenemyObject _returnvalue_2 _returnvalue_3))
        (Variables|/Game/BlueprintsAndMaps/Blueprints/EnemyBPs/enemyObject_BP.enemyObject_BP_C|SetenemyDataStructure _output_get _returnvalue)
        (Default|SetEnemytoOverWorldState _returnvalue_2)
        (Default|UpdateEnemyREFfromStats _returnvalue_2))))
  (return))

(fn SpawnSingleEnemyatDefaultLocation
  (params (enemyName :type Name))
  (bind _returnvalue (Game|GetPlayerCharacter 0))
  (bind _returnvalue_2 (Transformation|GetActorLocation _returnvalue))
  (bind _returnvalue_3 (Utilities|GetDataTableRow "/Game/BlueprintsAndMaps/Blueprints/EnemyBPs/EnemyDataTable.EnemyDataTable" enemyName)
    (:then
      (bind _returnvalue_4 (Game|SpawnActorfromClass (.enemyClass (Utilities|Struct|BreakEnemyDataStructure _returnvalue_3)) (Math|Transform|MakeTransform (Math|Vector|MakeVector (+ (.x _returnvalue_2) (Math|Random|RandomFloatinRange -5e+02 5e+02)) (+ (.y _returnvalue_2) (Math|Random|RandomFloatinRange -5e+02 5e+02)) (.z _returnvalue_2)) "0,180.000000, 0") "AdjustIfPossibleButAlwaysSpawn" 0 0 0))
      (bind _output_get (LocalVariables|SetRETenemiesToAdd _returnvalue_4))
      (bind _returnvalue_5 (Game|ConstructObjectfromClass "/Game/BlueprintsAndMaps/Blueprints/EnemyBPs/enemyObject_BP.enemyObject_BP_C" _output_get))
      (bind _output_get_2 (Variables|/Game/BlueprintsAndMaps/Blueprints/EnemyBPs/Demo_BPs/overWorldEnemyPawnBP.overWorldEnemyPawnBP_C|SetenemyObject (LocalVariables|GetRETenemiesToAdd) _returnvalue_5))
      (Variables|/Game/BlueprintsAndMaps/Blueprints/EnemyBPs/enemyObject_BP.enemyObject_BP_C|SetenemyDataStructure _output_get_2 _returnvalue_3)
      (Default|SetEnemytoOverWorldState (LocalVariables|GetRETenemiesToAdd))
      (Default|UpdateEnemyREFfromStats (LocalVariables|GetRETenemiesToAdd))
      (return (Variables|/Game/BlueprintsAndMaps/Blueprints/EnemyBPs/enemyObject_BP.enemyObject_BP_C|GetenemyDataStructure (Variables|/Game/BlueprintsAndMaps/Blueprints/EnemyBPs/Demo_BPs/overWorldEnemyPawnBP.overWorldEnemyPawnBP_C|GetenemyObject (LocalVariables|GetRETenemiesToAdd))) (LocalVariables|GetRETenemiesToAdd)))))

(fn SetLoadedEnemiesbyActiveMobSpawns
  (params (activeMobSpawns :type Array%20of%20Enemy%20Data%20Structure%20Structures))
  (Utilities|Array|Clear (Variables|Default|GetLoadedEnemiesByName))
  (for _array_element activeMobSpawns
    (Utilities|Array|Add (Variables|Default|GetLoadedEnemiesByName) (Utilities|String|StringToName (.enemyName (Utilities|Struct|BreakEnemyDataStructure _array_element)))))
  (return))

(fn SetMaxHponLevel
  (bind _maingameinstanceplayerobjectbp (Variables|Default|GetMainGameInstancePlayerObjectBP))
  (bind _output_get (Variables|/Game/BlueprintsAndMaps/Blueprints/PlayerBPs/playerObjectBP.playerObjectBP_C|SetREFPlayerMaxHealth _maingameinstanceplayerobjectbp (Utilities|Array|Get(acopy) (Variables|Default|GetmaxHpOnLvl) (- (Variables|/Game/BlueprintsAndMaps/Blueprints/PlayerBPs/playerObjectBP.playerObjectBP_C|GetREFPlayerLevel (Variables|Default|GetMainGameInstancePlayerObjectBP)) 1))))
  (Variables|/Game/BlueprintsAndMaps/Blueprints/PlayerBPs/playerObjectBP.playerObjectBP_C|SetREFPlayerCurrentHealth _maingameinstanceplayerobjectbp _output_get))

(fn SetExptoNextLevel
  (bind _maingameinstanceplayerobjectbp (Variables|Default|GetMainGameInstancePlayerObjectBP))
  (bind _maingameinstanceplayerobjectbp_2 (Variables|Default|GetMainGameInstancePlayerObjectBP))
  (bind _refplayerlevel (Variables|/Game/BlueprintsAndMaps/Blueprints/PlayerBPs/playerObjectBP.playerObjectBP_C|GetREFPlayerLevel _maingameinstanceplayerobjectbp))
  (bind _returnvalue (- _refplayerlevel 1))
  (Variables|/Game/BlueprintsAndMaps/Blueprints/PlayerBPs/playerObjectBP.playerObjectBP_C|SetREFPlayerExpToNextLevel _maingameinstanceplayerobjectbp_2 (Utilities|Array|Get(acopy) (Variables|Default|GetexpToNextLevelLIst) _returnvalue))
  (if (> _returnvalue 0)
    (Variables|/Game/BlueprintsAndMaps/Blueprints/PlayerBPs/playerObjectBP.playerObjectBP_C|SetREFPlayerPreviousExpToNextLevel _maingameinstanceplayerobjectbp_2 (Utilities|Array|Get(acopy) (Variables|Default|GetexpToNextLevelLIst) (- (Variables|/Game/BlueprintsAndMaps/Blueprints/PlayerBPs/playerObjectBP.playerObjectBP_C|GetREFPlayerLevel (Variables|Default|GetMainGameInstancePlayerObjectBP)) 2)))
    (else
      (Variables|/Game/BlueprintsAndMaps/Blueprints/PlayerBPs/playerObjectBP.playerObjectBP_C|SetREFPlayerPreviousExpToNextLevel (Variables|Default|GetMainGameInstancePlayerObjectBP) 0))))

(fn SetEnemyLoot
  (bind _currentenemyexpondefeat (Variables|Default|GetcurrentEnemyExpOnDefeat))
  (bind _currentbattleenemyoverworlddata (Variables|Default|GetcurrentBattleEnemyOverworldData))
  (bind _enemyobject (Variables|/Game/BlueprintsAndMaps/Blueprints/EnemyBPs/Demo_BPs/overWorldEnemyPawnBP.overWorldEnemyPawnBP_C|GetenemyObject _currentbattleenemyoverworlddata))
  (bind _enemydatastructure (Variables|/Game/BlueprintsAndMaps/Blueprints/EnemyBPs/enemyObject_BP.enemyObject_BP_C|GetenemyDataStructure _enemyobject))
  (Utilities|Array|SetArrayElem _currentenemyexpondefeat 0 (.minexperience (.enemylootstructure _enemydatastructure)))
  (Utilities|Array|SetArrayElem _currentenemyexpondefeat 1 (.maxexperience (.enemylootstructure _enemydatastructure))))

(fn DestroyPlayerLocators
  (bind _asplayer_controller_bp (Utilities|Casting|CastToplayerControllerBP (Game|GetPlayerController 0)))
  (Variables|/Game/BlueprintsAndMaps/Blueprints/PlayerBPs/playerControllerBP.playerControllerBP_C|SetlaunchedPlayer _asplayer_controller_bp false)
  (Variables|/Game/BlueprintsAndMaps/Blueprints/PlayerBPs/playerControllerBP.playerControllerBP_C|SethasSpawnedLocatorOrIndicator _asplayer_controller_bp false)
  (Variables|/Game/BlueprintsAndMaps/Blueprints/PlayerBPs/playerControllerBP.playerControllerBP_C|SetisAttemptingDash _asplayer_controller_bp false)
  (Variables|/Game/BlueprintsAndMaps/Blueprints/PlayerBPs/playerControllerBP.playerControllerBP_C|SetcanMove _asplayer_controller_bp true)
  (bind _asoverworld_player_bp (Utilities|Casting|CastTooverworldPlayerBP (Game|GetPlayerCharacter 0)))
  (Variables|/Game/BlueprintsAndMaps/Blueprints/PlayerBPs/overworldPlayerBP.overworldPlayerBP_C|SetisSpecialAttacking _asoverworld_player_bp false)
  (Variables|/Game/BlueprintsAndMaps/Blueprints/PlayerBPs/overworldPlayerBP.overworldPlayerBP_C|SetisDashing _asoverworld_player_bp false)
  (Variables|/Game/BlueprintsAndMaps/Blueprints/PlayerBPs/overworldPlayerBP.overworldPlayerBP_C|SetisBouncing _asoverworld_player_bp false)
  (bind _outactors (Actor|GetAllActorsOfClass "/Game/BlueprintsAndMaps/Blueprints/PlayerBPs/DemoBPs/slingshotLocator.slingshotLocator_C"))
  (Utilities|IsValid (Utilities|Array|Get(acopy) _outactors)
    (:Is%20Valid
      (for _array_element _outactors
        (Actor|DestroyActor _array_element)))
    (:Is%20Not%20Valid
      (bind _outactors_2 (Actor|GetAllActorsOfClass "/Game/BlueprintsAndMaps/Blueprints/PlayerBPs/DemoBPs/dashLocator.dashLocator_C"))
      (Utilities|IsValid (Utilities|Array|Get(acopy) _outactors_2)
        (:Is%20Valid
          (for _array_element_2 _outactors_2
            (Actor|DestroyActor _array_element_2)))
        (:Is%20Not%20Valid
          (bind _outactors_3 (Actor|GetAllActorsOfClass "/Game/BlueprintsAndMaps/Blueprints/PlayerBPs/DemoBPs/onHoverLocator.onHoverLocator_C"))
          (for _array_element_3 _outactors_3
            (Actor|DestroyActor _array_element_3)))))))

(fn SetQuestEventFlags
  (params (savedQuestEvents :type Array%20of%20Booleans))
  (Variables|Default|SetREFplayerQuestEvents savedQuestEvents))