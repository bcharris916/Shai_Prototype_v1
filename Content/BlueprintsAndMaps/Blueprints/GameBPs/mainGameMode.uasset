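; Overworld game mode that handles player spawn placement, the overworld UI and the transition into battles.
; On BeginPlay it activates the spawn gate matching the game instance's saved enum and adds the UI.
; sendToBattle saves camera and player positions, then opens BattleMap behind a start screen, or ends battle if the enemy is invalid or defeated.
; It also shows the end-battle screen; enemy spawning and per-area battle map selection are unhooked.
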(event Custom|spawnNewEnemy
  ;[1 0 0] UNHOOKED CURRENTLY!!Game Mode can Spawn new Enemies and takes a Spawn Origin point(middle of tile) and from a given Spawn Radius, picks a random point and random rotation to Spawn in Overworld.
)

(event Custom|sendToBattle
  (bind _returnvalue (Game|GetGameInstance))
  (bind _asmain_game_instance (Utilities|Casting|CastTomainGameInstance _returnvalue))
  (bind _currentbattleenemyoverworlddata (Variables|/Game/BlueprintsAndMaps/Blueprints/GameBPs/mainGameInstance.mainGameInstance_C|GetcurrentBattleEnemyOverworldData _asmain_game_instance))
  ;[1 1 1] Game Mode sends Player To BattleMap and stores the Camera and Players positions to spawn them there after Battle.
  (Utilities|FlowControl|Delay (Variables|Default|GetOverworldToBattleMapDelay))
  (bind _outactors (Actor|GetAllActorsOfClass "/Game/BlueprintsAndMaps/Blueprints/PlayerBPs/OverworldCameaBP.OverworldCameaBP_C"))
  (Variables|/Game/BlueprintsAndMaps/Blueprints/GameBPs/mainGameInstance.mainGameInstance_C|SetoverworldCameraOrigin (.AsMain%20Game%20Instance (Utilities|Casting|CastTomainGameInstance (Game|GetGameInstance))) (Transformation|GetActorLocation (Utilities|Array|Get(acopy) _outactors)))
  (Variables|/Game/BlueprintsAndMaps/Blueprints/GameBPs/mainGameInstance.mainGameInstance_C|SetoverworldPlayerOrigin (.AsMain%20Game%20Instance (Utilities|Casting|CastTomainGameInstance (Game|GetGameInstance))) (Transformation|GetActorLocation (Game|GetPlayerCharacter 0)))
  (Utilities|IsValid _currentbattleenemyoverworlddata
    (:Is%20Valid
      (if (Variables|/Game/BlueprintsAndMaps/Blueprints/EnemyBPs/Demo_BPs/overWorldEnemyPawnBP.overWorldEnemyPawnBP_C|GetisDefeated _currentbattleenemyoverworlddata)
        (Default|EndBattle _asmain_game_instance :!label _label)
        (else
          (Variables|/Game/BlueprintsAndMaps/Blueprints/GameBPs/mainGameInstance.mainGameInstance_C|SetisBattle? _asmain_game_instance true)
          (bind _returnvalue_2 (UserInterface|CreateWidget "/Game/BlueprintsAndMaps/Blueprints/UI_BPs/DemoBPs/battleStartScreen.battleStartScreen_C" (Game|GetPlayerController 0)))
          (UserInterface|Viewport|AddtoViewport _returnvalue_2 0)
          (Utilities|FlowControl|Delay (Variables|Default|GetOverworldToBattleMapDelay))
          (Game|OpenLevel(byName) "BattleMap"))))
    (:Is%20Not%20Valid
      (goto _label))))

(event Custom|displayEndBattleScreen
  (bind _returnvalue (UserInterface|CreateWidget "/Game/BlueprintsAndMaps/Blueprints/UI_BPs/DemoBPs/endBattleScreen.endBattleScreen_C" (Game|GetPlayerController 0)))
  (Variables|Default|SetcurrentEndBattleScreen _returnvalue)
  (UserInterface|Viewport|AddtoViewport (Variables|Default|GetcurrentEndBattleScreen) 0))

(event EventBeginPlay
  ;[1 1 1] On Game Mode Begin Play, Add Overworld UI, set it locally and Add it to viewport. Set REf to Game Instance
  (bind _outactors (Actor|GetAllActorsOfClass "/Game/BlueprintsAndMaps/Blueprints/WorldBPs/spawnGateActor.spawnGateActor_C"))
  (CallFunction|ChooseSpawnGate _outactors)
  (bind _returnvalue (UserInterface|CreateWidget "/Game/BlueprintsAndMaps/Blueprints/UI_BPs/OverworldUI.OverworldUI_C" (Game|GetPlayerController 0)))
  (bind _output_get (Variables|Default|SetcurrentOverworldUI _returnvalue))
  (UserInterface|Viewport|AddtoViewport _output_get 0)
  (bind _asmain_game_instance (Utilities|Casting|CastTomainGameInstance (Game|GetGameInstance)))
  (Variables|Default|SetREF_MainGameInstance _asmain_game_instance))

(fn ConstructionScript)

(fn ChooseSpawnGate
  (params (allSpawnGates :type Array%20of%20Spawn%20Gate%20Actor%20Object%20References))
  (bind _array_element (Utilities|Array|ForEachLoopwithBreak allSpawnGates :!label _label)
    (:LoopBody
      (bind _asmain_game_instance (Utilities|Casting|CastTomainGameInstance (Game|GetGameInstance)))
      (if (Utilities|Enum|Equal(Enum) (Variables|/Game/BlueprintsAndMaps/Blueprints/GameBPs/mainGameInstance.mainGameInstance_C|GetplayerShouldSpawnHere _asmain_game_instance) (Variables|/Game/BlueprintsAndMaps/Blueprints/WorldBPs/spawnGateActor.spawnGateActor_C|GetmyGateEnum _array_element))
        (goto _label Break)))
    (:Completed
      (bind _output_get (Variables|Default|SetplayerSpawnGate _array_element))
      (Default|PlayerSpawnedHere _output_get)
      (return))))