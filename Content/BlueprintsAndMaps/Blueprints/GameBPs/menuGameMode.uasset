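; Game mode for the main menu that starts the menu music and handles starting or loading a game.
; On BeginPlay it caches the main game instance and tells it to play the menu theme.
; Separate events create and show the new-game and load-save widgets.
; NewGame resets player data through the game instance before opening the overworld map, while LoadGame just opens that map.
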(event Custom|addNewGameWindow
  (bind _returnvalue (UserInterface|CreateWidget "/Game/BlueprintsAndMaps/Blueprints/UI_BPs/MainMenu_NewGame.MainMenu_NewGame_C"))
  (bind _output_get (Variables|Default|SetREFMainMenuNewGameWidget _returnvalue))
  (UserInterface|Viewport|AddtoViewport _output_get 0))

(event Custom|LoadGame
  (Game|OpenLevel(byName) (Variables|Default|GetOverWorldMapName)))

(event Custom|addLoadSaveWindow
  (bind _returnvalue (UserInterface|CreateWidget "/Game/BlueprintsAndMaps/Blueprints/UI_BPs/MainMenu_LoadSave.MainMenu_LoadSave_C"))
  (bind _output_get (Variables|Default|SetREFMainMenuLoadSaveWidget _returnvalue))
  (UserInterface|Viewport|AddtoViewport _output_get 0))

(event Custom|NewGame
  (Default|UpdatePlayerNewGame (Variables|Default|GetREFMainGameInstance))
  (Game|OpenLevel(byName) (Variables|Default|GetOverWorldMapName)))

(event EventBeginPlay
  (bind _asmain_game_instance (Utilities|Casting|CastTomainGameInstance (Game|GetGameInstance)))
  (bind _output_get (Variables|Default|SetREFMainGameInstance _asmain_game_instance))
  (Default|PlayMenuTheme _output_get))

(event EventTick
  (params (DeltaSeconds :type Float%20%28single-precision%29)))

(fn ConstructionScript)