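; Player pawn for battles that shows the character with its equipped weapon and tracks health during combat.
; On BeginPlay it sockets face, head, shoe and weapon meshes, caches the Game Instance's player object and signals the battle Game Mode that the player's turn finished.
; Damage and capped recharge healing write health back to that player object.
; Damage also notifies the battle UI and triggers the revive state on defeat.
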(event Custom|takeDamage
  (params (damageTaken :type Integer))
  ;[1 1 1] Player Takes Damage. Subtract incoming damage from Players current HP
  (bind _newcurrenthealth (CallFunction|UpdatePlayerHealthonDamage damageTaken))
  (Variables|Default|SetplayerCurrentHealth (Math|Conversions|ToFloat(Integer) _newcurrenthealth))
  ;[1 1 1] To display the Damage dealt we let the Game Modes current Battle UI know the Damage amount.
  (bind _asbattle_game_mode (Utilities|Casting|CastTobattleGameMode (Game|GetGameMode)))
  (Default|PlayerTakesDamage (Variables|/Game/BlueprintsAndMaps/Blueprints/GameBPs/battleGameMode.battleGameMode_C|GetcurrentBattleUIInstance _asbattle_game_mode) damageTaken)
  ;[1 1 1] Check if dead and update current values from damage to Game Instance
  (CallFunction|UpdatePlayerHealthonPlayerObject (<= (Variables|Default|GetplayerCurrentHealth) 0.0)))

(event Custom|updatePlayerHealthOnPlayerObject
  (params (wasPlayerDefeated :type Boolean))
  ;[1 1 1] Update Player Statuses on Player Object
  (bind _asmain_game_instance (Utilities|Casting|CastTomainGameInstance (Game|GetGameInstance)))
  (Variables|/Game/BlueprintsAndMaps/Blueprints/PlayerBPs/playerObjectBP.playerObjectBP_C|SetREFPlayerCurrentHealth (Variables|/Game/BlueprintsAndMaps/Blueprints/GameBPs/mainGameInstance.mainGameInstance_C|GetMainGameInstancePlayerObjectBP _asmain_game_instance) (Math|Float|Truncate (Variables|Default|GetplayerCurrentHealth)))
  (Default|UpdatePlayerStatsStructurefromREF (Variables|/Game/BlueprintsAndMaps/Blueprints/GameBPs/mainGameInstance.mainGameInstance_C|GetMainGameInstancePlayerObjectBP _asmain_game_instance))
  (bind _output_get (Variables|/Game/BlueprintsAndMaps/Blueprints/GameBPs/mainGameInstance.mainGameInstance_C|SetplayerDefeated _asmain_game_instance wasPlayerDefeated))
  (if _output_get
    (Default|SetPlayertoReviveState _asmain_game_instance)))

(event Custom|updatePlayerHealthFromRecharge
  (params (changedHealth :type Integer))
  ;[1 1 1] Event called to Update Players Health for Recharge Ability.  This could possibly be merged with Take Damage in such a way that we could add or subtract HP there and know the condition and dam,age dealr/healing source.
  (Variables|Default|SetplayerCurrentHealth (Math|Conversions|ToFloat(Integer) (Variables|/Game/BlueprintsAndMaps/Blueprints/PlayerBPs/playerObjectBP.playerObjectBP_C|GetREFPlayerCurrentHealth (Variables|Default|GetREFPlayerObject))))
  (Variables|Default|SetplayerMaxHealth (Math|Conversions|ToFloat(Integer) (Variables|/Game/BlueprintsAndMaps/Blueprints/PlayerBPs/playerObjectBP.playerObjectBP_C|GetREFPlayerMaxHealth (Variables|Default|GetREFPlayerObject))))
  (if (>= (+ (Math|Conversions|ToFloat(Integer) changedHealth) (Variables|Default|GetplayerCurrentHealth)) (Variables|Default|GetplayerMaxHealth))
    (Variables|Default|SetplayerCurrentHealth (Variables|Default|GetplayerMaxHealth))
    (else
      (Variables|Default|SetplayerCurrentHealth (+ (Math|Conversions|ToFloat(Integer) changedHealth) (Variables|Default|GetplayerCurrentHealth)))))
  (CallFunction|UpdatePlayerHealthonPlayerObject false))

(event EventBeginPlay
  ;[1 1 1] At Begin Play attach face decal mesh to Player Pawn. Then update the Player from the Game Instance with Statuses
  (Transformation|AttachComponentToComponent (Variables|Default|GetFaceMesh) (Variables|Character|GetMesh) "FaceSocket" "SnapToTarget" "SnapToTarget" "SnapToTarget" true)
  (CallFunction|SetWeaponMesh)
  ;[1 1 1] Attach Demo Weapon to Mesh at Named Socket
  (Transformation|AttachComponentToComponent (Variables|Default|GetWeaponMesh) (Variables|Character|GetMesh) "WeaponSocket" "SnapToTarget" "SnapToTarget" "SnapToTarget" true)
  (Transformation|AttachComponentToComponent (Variables|Default|GetR_ShoeMesh) (Variables|Character|GetMesh) "RightFootSocket" "SnapToTarget" "SnapToTarget" "SnapToTarget" true)
  (Transformation|AttachComponentToComponent (Variables|Default|GetL_ShoeMesh) (Variables|Character|GetMesh) "LeftFootSocket" "SnapToTarget" "SnapToTarget" "SnapToTarget" true)
  (Transformation|AttachComponentToComponent (Variables|Default|GetHeadMesh) (Variables|Character|GetMesh) "HeadSocket" "SnapToTarget" "SnapToTarget" "SnapToTarget" true)
  (bind _asbattle_game_mode (Utilities|Casting|CastTobattleGameMode (Game|GetGameMode)))
  (bind _asmain_game_instance (Utilities|Casting|CastTomainGameInstance (Game|GetGameInstance)))
  (Variables|Default|SetREFPlayerObject (Variables|/Game/BlueprintsAndMaps/Blueprints/GameBPs/mainGameInstance.mainGameInstance_C|GetMainGameInstancePlayerObjectBP _asmain_game_instance))
  (Default|PlayerFinishedTurn _asbattle_game_mode))

(fn ConstructionScript)

(fn UpdatePlayerHealthonDamage
  (params (damageTaken :type Integer))
  (return (- (Variables|/Game/BlueprintsAndMaps/Blueprints/PlayerBPs/playerObjectBP.playerObjectBP_C|GetREFPlayerCurrentHealth (Variables|Default|GetREFPlayerObject)) damageTaken)))

(fn SetWeaponMesh
  (bind _returnvalue (Game|GetGameInstance))
  (bind _asmain_game_instance (Utilities|Casting|CastTomainGameInstance _returnvalue))
  (bind _maingameinstanceplayerobjectbp (Variables|/Game/BlueprintsAndMaps/Blueprints/GameBPs/mainGameInstance.mainGameInstance_C|GetMainGameInstancePlayerObjectBP _asmain_game_instance))
  (bind _refplayerallweapons (Variables|/Game/BlueprintsAndMaps/Blueprints/PlayerBPs/playerObjectBP.playerObjectBP_C|GetREFPlayerAllWeapons _maingameinstanceplayerobjectbp))
  (bind _output (Utilities|Array|Get(acopy) _refplayerallweapons))
  (Utilities|IsValid (.weaponmodel _output)
    (:Is%20Valid
      (Components|StaticMesh|SetStaticMesh (Variables|Default|GetWeaponMesh) (.weaponmodel _output)))))