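; Player controller for turn-based battles that turns mouse swipes into player actions during the player's turn.
; Left-button press and release deltas are compared against a threshold to pick one direction, ignoring short or diagonal drags.
; A valid swipe opens a Tick-driven gate that sets battlePlayerBP action flags for defend, basic attack, special attack or recharge.
; The game instance's player object energy-checks all but defend, and recharge also updates health and ends the turn.
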(event Custom|InputRegistered
  ;[1 1 1] Enter Gate on Event Tick and Open it When  an Input is registered from Left Mosue Button Event.
  (if (Variables|Default|GetplayerTurn)
    (Utilities|FlowControl|Gate true) ; enters at Open
  ))

(event EventBeginPlay
  ;[1 1 1] On Battle Controller Begin Play Show Mouse Cursor
  (Variables|Default|SetbShowMouseCursor true)
  (bind _asmain_game_instance (Utilities|Casting|CastTomainGameInstance (Game|GetGameInstance)))
  (bind _output_get (Variables|Default|SetmyMainGameInstance _asmain_game_instance))
  (Variables|Default|SetmyMainPlayerObject (Variables|/Game/BlueprintsAndMaps/Blueprints/GameBPs/mainGameInstance.mainGameInstance_C|GetMainGameInstancePlayerObjectBP _output_get)))

(event EventTick
  (params (DeltaSeconds :type Float%20%28single-precision%29))
  ;[1 1 1] Enter Gate on Event Tick and Open it When  an Input is registered from Left Mosue Button Event.
  (Utilities|FlowControl|Gate true :!label _label
    (:Exit
      ;[1 1 1] Depending on the Input that was registered and ccording flag set, set the appropriate flag for the Anim BP to carry out an Animation and from there reset this flag.
      (if (Variables|Default|GetisSwipeLeft)
        (Variables|/Game/BlueprintsAndMaps/Blueprints/PlayerBPs/battlePlayerBP.battlePlayerBP_C|SetisDefending (.AsBattle%20Player%20BP (Utilities|Casting|CastTobattlePlayerBP (Game|GetPlayerCharacter 0))) true)
        (goto _label Close)
        (elif (Variables|Default|GetisSwipeRight)
          (bind _canuseskill (Default|CheckEnergy (Variables|Default|GetmyMainPlayerObject) "NewEnumerator0"))
          (Variables|/Game/BlueprintsAndMaps/Blueprints/PlayerBPs/battlePlayerBP.battlePlayerBP_C|SetisBasicAttacking (.AsBattle%20Player%20BP (Utilities|Casting|CastTobattlePlayerBP (Game|GetPlayerCharacter 0))) _canuseskill)
          (goto _label Close)
          (elif (Variables|Default|GetisSwipeDown)
            (bind _canuseskill_2 (Default|CheckEnergy (Variables|Default|GetmyMainPlayerObject) "NewEnumerator2"))
            (if _canuseskill_2
              (Variables|/Game/BlueprintsAndMaps/Blueprints/PlayerBPs/battlePlayerBP.battlePlayerBP_C|SetisRecharging (.AsBattle%20Player%20BP (Utilities|Casting|CastTobattlePlayerBP (Game|GetPlayerCharacter 0))) _canuseskill_2)
              (bind _asmain_game_instance (Utilities|Casting|CastTomainGameInstance (Game|GetGameInstance)))
              (Default|UpdatePlayerHealthfromRecharge (Variables|/Game/BlueprintsAndMaps/Blueprints/GameBPs/mainGameInstance.mainGameInstance_C|GetMainGameInstancePlayerObjectBP _asmain_game_instance))
              (Default|UpdatePlayerStatsStructurefromREF (Variables|/Game/BlueprintsAndMaps/Blueprints/GameBPs/mainGameInstance.mainGameInstance_C|GetMainGameInstancePlayerObjectBP _asmain_game_instance))
              (Variables|Default|SetplayerTurn false)
              (goto _label Close)
              (else
                (goto _label Close)))
            (elif (Variables|Default|GetisSwipeUp)
              (bind _canuseskill_3 (Default|CheckEnergy (Variables|Default|GetmyMainPlayerObject) "NewEnumerator1"))
              (Variables|/Game/BlueprintsAndMaps/Blueprints/PlayerBPs/battlePlayerBP.battlePlayerBP_C|SetisSpecialAttacking (.AsBattle%20Player%20BP (Utilities|Casting|CastTobattlePlayerBP (Game|GetPlayerCharacter 0))) _canuseskill_3)
              (goto _label Close))))))))

(event Input|MouseEvents|LeftMouseButton
  (params (Key :type Key%20Structure :default "None"))
  (bind (_locationx _locationy) (Game|Player|GetMousePosition))
  (bind (_locationx_2 _locationy_2) (Game|Player|GetMousePosition))
  ;[1 1 1] On Mouse Press, ensure it is Players Turn
  (:Pressed
    (if (Variables|Default|GetplayerTurn)
      ;[1 1 1] Reset all Swipe flags
      (Variables|Default|SetnoSwipe false)
      (Variables|Default|SetisSwipeUp false)
      (Variables|Default|SetisSwipeRight false)
      (Variables|Default|SetisSwipeDown false)
      ;[1 1 1] Get Screen Pos. of Mouse click on Press
      (Variables|Default|SetisSwipeLeft false)
      (Variables|Default|SetclickedX _locationx_2)
      (Variables|Default|SetclickedY _locationy_2)))
  (:Released
    (if (Variables|Default|GetplayerTurn)
      ;[1 1 1] On Mouse release, check Delta of Mouse position and see if Swipe was registered.  If so set its Flag and call Input Registered.
      (Variables|Default|SetreleasedX _locationx)
      (Variables|Default|SetreleasedY _locationy)
      (if (< (- (Variables|Default|GetreleasedY) (Variables|Default|GetclickedY)) 0.0)
        (Variables|Default|SetdeltaY (* (- (Variables|Default|GetreleasedY) (Variables|Default|GetclickedY)) -1.0))
        (Variables|Default|SetisSwipeUp true)
        (else
          (Variables|Default|SetdeltaY (- (Variables|Default|GetreleasedY) (Variables|Default|GetclickedY)))
          (Variables|Default|SetisSwipeDown true)))
      (if (< (- (Variables|Default|GetreleasedX) (Variables|Default|GetclickedX)) 0.0)
        (Variables|Default|SetdeltaX (* (- (Variables|Default|GetreleasedX) (Variables|Default|GetclickedX)) -1.0))
        (Variables|Default|SetisSwipeLeft true)
        (else
          (Variables|Default|SetdeltaX (- (Variables|Default|GetreleasedX) (Variables|Default|GetclickedX)))
          (Variables|Default|SetisSwipeRight true)))
      (if (<= (Variables|Default|GetdeltaX) (Variables|Default|GetvalueLimit))
        (if (<= (Variables|Default|GetdeltaY) (Variables|Default|GetvalueLimit))
          (Variables|Default|SetnoSwipe true)
          (else
            (if (Variables|Default|GetisSwipeDown)
              _
              (else
                _))
            (Variables|Default|SetisSwipeRight false)
            (Variables|Default|SetisSwipeLeft false)
            (CallFunction|InputRegistered :!label _label)))
        (elif (<= (Variables|Default|GetdeltaY) (Variables|Default|GetvalueLimit))
          (if (Variables|Default|GetisSwipeLeft)
            _
            (else
              _))
          (Variables|Default|SetisSwipeDown false)
          (Variables|Default|SetisSwipeUp false)
          (goto _label))))))

(fn ConstructionScript)