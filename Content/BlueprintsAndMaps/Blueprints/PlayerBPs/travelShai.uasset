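; Player-character Blueprint for Shai that shows the assembled character in a looping travel animation.
; On BeginPlay it snaps separate weapon, left and right shoe, and head meshes to named sockets on the main skeletal mesh.
; It then plays ShaiTravelAnim directly on that mesh, with no other active logic in the graph.
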(event EventBeginPlay
  ;[1 1 1] Attaches Face Mesh to Player Character
  ;[1 1 1] Attach Demo Weapon to Mesh at Named Socket
  (Transformation|AttachComponentToComponent (Variables|Default|GetWeaponMesh) (Variables|Default|GetMesh) "WEaponSocket" "SnapToTarget" "SnapToTarget" "SnapToTarget" true)
  (Transformation|AttachComponentToComponent (Variables|Default|GetR_ShoeMesh) (Variables|Default|GetMesh) "RightFootSocket" "SnapToTarget" "SnapToTarget" "SnapToTarget" true)
  (Transformation|AttachComponentToComponent (Variables|Default|GetL_ShoeMesh) (Variables|Default|GetMesh) "LeftFootSocket" "SnapToTarget" "SnapToTarget" "SnapToTarget" true)
  (Transformation|AttachComponentToComponent (Variables|Default|GetHeadMesh) (Variables|Default|GetMesh) "HeadSocket" "SnapToTarget" "SnapToTarget" "SnapToTarget" true)
  (Components|Animation|PlayAnimation (Variables|Default|GetMesh) "/Game/myModels/ShaiAnims/ShaiTravelAnim.ShaiTravelAnim" true))

(event EventTick
  (params (DeltaSeconds :type Float%20%28single-precision%29)))

(event Collision|EventActorBeginOverlap
  (params (OtherActor :type Actor%20Object%20Reference)))

(fn ConstructionScript)