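; Player data object that holds stats, skills, weapons and resources, and handles power, damage, recharge healing and energy costs.
; REF working variables sync with PlayerStatsStructure, which is also updated from save data.
; Skills and weapons are added by DataTable row name, with equipped skills in fixed slots by type and index 0 as the equipped weapon.
; Total power combines level, base power and weapon bonus in a log-scaled formula that drives randomized skill damage.
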(event Custom|updatePlayerStatsStructureFromREF
  ;[1 1 1] Event called when the REF variables have the data the Player Structure needs.
  (Variables|Default|SetplayerStatsStructure (Utilities|Struct|MakePlayerStatsStructure (Variables|Default|GetREFPlayerCurrentHealth) (Variables|Default|GetREFPlayerMaxHealth) (Variables|Default|GetREFPlayerCurrentExp) (Variables|Default|GetREFPlayerExpToNextLevel) (Variables|Default|GetREFPlayerLevel) (Variables|Default|GetREFBasePowerLevel) (Variables|Default|GetREFProfileName) (Variables|Default|GetREFPlayerSaveSlot) (Variables|Default|GetREFPlayerPreviousExpToNextLevel) (Variables|Default|GetREFCurrentLevelName) (Variables|Default|GetREFPlayerAllWeapons) (Variables|Default|GetREFPlayerAllSkills) (Variables|Default|GetREFPlayerEquippedSkills) (Variables|Default|GetREFPlayerCurrentEnergy) (Variables|Default|GetREFPlayerMaxEnergy))))

(event Custom|updatePlayerStatsStructureFromSaveGameObject
  (params (loadedPlayerStatsStructure :type Player%20Stats%20Structure%20Structure))
  ;[1 1 1] Event called when player loads a saved game to retrieve the Player Stats Structure from the Saved Game Object.
  (Variables|Default|SetplayerStatsStructure loadedPlayerStatsStructure)
  (CallFunction|LoadWEaponsIntoStruct)
  (CallFunction|LoadAllSkillsIntoStruct)
  (CallFunction|LoadEquippedSkillsIntoStruct)
  (CallFunction|UpdateREFVariablesfromPlayerStatsStructure))

(event Custom|loadEquippedSkillsIntoREF
  (Variables|Default|SetREFSkillsToEquip (.playerEquippedSkills (Utilities|Struct|BreakPlayerStatsStructure (Variables|Default|GetplayerStatsStructure))))
  (CallFunction|SetEquippedSkillstoSlots))

(event Custom|loadEquippedSkillsIntoStruct
  (Variables|Default|SetplayerStatsStructure (Utilities|Struct|MakePlayerStatsStructure (.playercurrenthealth (Variables|Default|GetplayerStatsStructure)) (.playermaxhealth (Variables|Default|GetplayerStatsStructure)) (.playerexp (Variables|Default|GetplayerStatsStructure)) (.playerexptonextlevel (Variables|Default|GetplayerStatsStructure)) (.playerlevel (Variables|Default|GetplayerStatsStructure)) (.playerbasepower (Variables|Default|GetplayerStatsStructure)) (.profilename (Variables|Default|GetplayerStatsStructure)) (.playersaveslot (Variables|Default|GetplayerStatsStructure)) (.previousplayerexptonextlevel (Variables|Default|GetplayerStatsStructure)) (.currentlevelname (Variables|Default|GetplayerStatsStructure)) (.playerallweapons (Variables|Default|GetplayerStatsStructure)) (.playerallskills (Variables|Default|GetplayerStatsStructure)) (Variables|Default|GetREFPlayerEquippedSkills) (.playercurrentenergy (Variables|Default|GetplayerStatsStructure)) (.playermaxenergy (Variables|Default|GetplayerStatsStructure)))))

(event Custom|addSkillToEquippedByData
  (params (chosenSkillsToEquip :type Array%20of%20Skill%20Data%20Structure%20Structures))
  (for _array_element chosenSkillsToEquip
    (bind _returnvalue (Utilities|GetDataTableRow "/Game/BlueprintsAndMaps/Blueprints/WeaponAndSkillsBPs/SkillDataTable.SkillDataTable" (Utilities|String|StringToName (.SkillName (Utilities|Struct|BreakSkillDataStructure _array_element))))
      (:then
        (Utilities|Array|Add (Variables|Default|GetREFSkillsToEquip) _returnvalue))))
  (CallFunction|SetEquippedSkillstoSlots))

(event Custom|setEquippedSkillsToSlots
  (for _array_element (Variables|Default|GetREFSkillsToEquip)
    (CallFunction|EquipSkilltoSlot (.SkillType (Utilities|Struct|BreakSkillDataStructure _array_element)) _array_element)))

(event Custom|addSkillToEquippedByName
  (params (skillsByName :type Array%20of%20Names))
  (for _array_element skillsByName
    (bind _returnvalue (Utilities|GetDataTableRow "/Game/BlueprintsAndMaps/Blueprints/WeaponAndSkillsBPs/SkillDataTable.SkillDataTable" _array_element)
      (:then
        (Utilities|Array|Add (Variables|Default|GetREFSkillsToEquip) _returnvalue))))
  (CallFunction|SetEquippedSkillstoSlots))

(event Custom|updatePlayerHealthFromRecharge
  (bind _rechargehealamount (CallFunction|CalcRechargeHealAmount))
  (bind _output_get (Variables|Default|SetcurrentRechargeAmountToDisplay _rechargehealamount))
  (bind _output_get_2 (Variables|Default|SetcurrentHealthPlusRecharge (+ (Variables|Default|GetREFPlayerCurrentHealth) _output_get)))
  (if (>= _output_get_2 (Variables|Default|GetREFPlayerMaxHealth))
    (Variables|Default|SetREFPlayerCurrentHealth (Variables|Default|GetREFPlayerMaxHealth))
    (else
      (Variables|Default|SetREFPlayerCurrentHealth (Variables|Default|GetcurrentHealthPlusRecharge)))))

(event Custom|updateREFVariablesFromPlayerStatsStructure
  (bind _playerstatsstructure (Variables|Default|GetplayerStatsStructure))
  (bind _playerstatsstructure_2 (Variables|Default|GetplayerStatsStructure))
  (bind _playerstatsstructure_3 (Variables|Default|GetplayerStatsStructure))
  (bind _playerstatsstructure_4 (Variables|Default|GetplayerStatsStructure))
  (bind _playerstatsstructure_5 (Variables|Default|GetplayerStatsStructure))
  ;[1 1 1] Event called when the Player Structure has the data we need to reset the REF variables.
  (Variables|Default|SetREFPlayerCurrentHealth (.playercurrenthealth _playerstatsstructure_2))
  (Variables|Default|SetREFPlayerMaxHealth (.playermaxhealth _playerstatsstructure_2))
  (Variables|Default|SetREFPlayerCurrentExp (.playerexp _playerstatsstructure_3))
  (Variables|Default|SetREFPlayerExpToNextLevel (.playerexptonextlevel _playerstatsstructure_3))
  (Variables|Default|SetREFPlayerPreviousExpToNextLevel (.previousplayerexptonextlevel _playerstatsstructure_4))
  (Variables|Default|SetREFPlayerLevel (.playerlevel _playerstatsstructure_4))
  (Variables|Default|SetREFPlayerCurrentEnergy (.playercurrentenergy _playerstatsstructure_4))
  (Variables|Default|SetREFPlayerMaxEnergy (.playermaxenergy _playerstatsstructure_4))
  (Variables|Default|SetREFProfileName (.profilename _playerstatsstructure_5))
  (Variables|Default|SetREFPlayerSaveSlot (.playersaveslot _playerstatsstructure_5))
  (Variables|Default|SetREFCurrentLevelName (.currentlevelname _playerstatsstructure_5))
  (Variables|Default|SetREFPlayerAllSkills (.playerallskills _playerstatsstructure))
  (Variables|Default|SetREFPlayerAllWeapons (.playerallweapons _playerstatsstructure))
  (Variables|Default|SetREFBasePowerLevel (.playerbasepower _playerstatsstructure))
  (Variables|Default|SetREFPlayerEquippedSkills (.playerequippedskills _playerstatsstructure)))

(event Custom|constructNewInventoryObject
  ;[1 1 1] Prototype Inventory Creation. Will always pull default values from our Class Defaults of Player Inventory Object.
  (bind _returnvalue (Game|ConstructObjectfromClass "/Game/BlueprintsAndMaps/Blueprints/PlayerBPs/playerInventoryObjectBP.playerInventoryObjectBP_C" self))
  (Variables|Default|SetREFPlayerInventoryObject _returnvalue))

(event Custom|constructNewSkillObject
  ;[1 1 1] Prototype Skill  Object Creation. Will always pull default values from our Class Defaults of Player Skills Object.
  (bind _returnvalue (Game|ConstructObjectfromClass "/Game/BlueprintsAndMaps/Blueprints/PlayerBPs/playerSkillsObjectBP.playerSkillsObjectBP_C" self))
  (Variables|Default|SetREFPlayerSkillsObject _returnvalue))

(event Custom|playerAquiresWeapon
  (params (weaponByName :type Name))
  (CallFunction|AddWeapontoInventorybyName weaponByName)
  (CallFunction|SetTotalPower))

(event Custom|loadWeaponsIntoStruct
  (Variables|Default|SetplayerStatsStructure (Utilities|Struct|MakePlayerStatsStructure (.playercurrenthealth (Variables|Default|GetplayerStatsStructure)) (.playermaxhealth (Variables|Default|GetplayerStatsStructure)) (.playerexp (Variables|Default|GetplayerStatsStructure)) (.playerexptonextlevel (Variables|Default|GetplayerStatsStructure)) (.playerlevel (Variables|Default|GetplayerStatsStructure)) (.playerbasepower (Variables|Default|GetplayerStatsStructure)) (.profilename (Variables|Default|GetplayerStatsStructure)) (.playersaveslot (Variables|Default|GetplayerStatsStructure)) (.previousplayerexptonextlevel (Variables|Default|GetplayerStatsStructure)) (.currentlevelname (Variables|Default|GetplayerStatsStructure)) (Variables|Default|GetREFPlayerAllWeapons) (.playerallskills (Variables|Default|GetplayerStatsStructure)) (.playerequippedskills (Variables|Default|GetplayerStatsStructure)) (.playercurrentenergy (Variables|Default|GetplayerStatsStructure)) (.playermaxenergy (Variables|Default|GetplayerStatsStructure)))))

(event Custom|loadAllSkillsIntoStruct
  (Variables|Default|SetplayerStatsStructure (Utilities|Struct|MakePlayerStatsStructure (.playercurrenthealth (Variables|Default|GetplayerStatsStructure)) (.playermaxhealth (Variables|Default|GetplayerStatsStructure)) (.playerexp (Variables|Default|GetplayerStatsStructure)) (.playerexptonextlevel (Variables|Default|GetplayerStatsStructure)) (.playerlevel (Variables|Default|GetplayerStatsStructure)) (.playerbasepower (Variables|Default|GetplayerStatsStructure)) (.profilename (Variables|Default|GetplayerStatsStructure)) (.playersaveslot (Variables|Default|GetplayerStatsStructure)) (.previousplayerexptonextlevel (Variables|Default|GetplayerStatsStructure)) (.currentlevelname (Variables|Default|GetplayerStatsStructure)) (.playerallweapons (Variables|Default|GetplayerStatsStructure)) (Variables|Default|GetREFPlayerAllSkills) (.playerequippedskills (Variables|Default|GetplayerStatsStructure)) (.playercurrentenergy (Variables|Default|GetplayerStatsStructure)) (.playermaxenergy (Variables|Default|GetplayerStatsStructure)))))

(event Custom|playerAquiresSkill
  (params (skillsAquired :type Array%20of%20Names))
  (CallFunction|AddSkilltoAllSkillsbySkillName skillsAquired))

(fn ReturnPlayerSaveSlot
  (return (.PlayerSaveSlot (Utilities|Struct|BreakPlayerStatsStructure (Variables|Default|GetplayerStatsStructure)))))

(fn CalcDamageSkill
  (params (skillUsed :type Skill%20Data%20Structure%20Structure))
  (bind _skillstatsstructure (Utilities|Struct|BreakSkillDataStructure skillUsed))
  (bind (_mindamagepercent _maxdamagepercent) (Utilities|Struct|BreakSkillStatsStructure _skillstatsstructure))
  (bind _power (CallFunction|SetTotalPower))
  (return (Math|Float|Truncate (Math|Random|RandomFloatinRange (* _power _mindamagepercent) (* _power _maxdamagepercent)))))

(fn ReturnSkillbyType
  (params (skillType :type skillTypes%20Enum :default "NewEnumerator0"))
  (LocalVariables|SetdesiredSkillType skillType)
  (for _array_element (Variables|Default|GetREFPlayerAllSkills)
    (if (Utilities|Enum|Equal(Enum) (.SkillType (Utilities|Struct|BreakSkillDataStructure _array_element)) (LocalVariables|GetdesiredSkillType))
      (return _array_element))))

(fn AddWeapontoInventorybyName
  (params (weaponName :type Name))
  (bind _returnvalue (Utilities|GetDataTableRow "/Game/BlueprintsAndMaps/Blueprints/WeaponAndSkillsBPs/WeaponDataTable.WeaponDataTable" weaponName)
    (:then
      (Utilities|Array|Add (Variables|Default|GetREFPlayerAllWeapons) _returnvalue)
      (return (Variables|Default|GetREFPlayerAllWeapons)))))

(fn LoadInventory
  (params (playerInventory :type Array%20of%20Weapon%20Data%20Structure%20Structures))
  (for _array_element playerInventory
    (CallFunction|AddWeapontoInventorybyName (Utilities|String|StringToName (.WeaponName (Utilities|Struct|BreakWeaponDataStructure _array_element)))))
  (return))

(fn AddSkilltoAllSkillsbySkillName
  (params (skillNames :type Array%20of%20Names))
  (for _array_element skillNames
    (bind _returnvalue (Utilities|GetDataTableRow "/Game/BlueprintsAndMaps/Blueprints/WeaponAndSkillsBPs/SkillDataTable.SkillDataTable" _array_element)
      (:then
        (Utilities|Array|Add (Variables|Default|GetREFPlayerAllSkills) _returnvalue))))
  (return))

(fn EquipSkilltoSlot
  (params (skillByType :type skillTypes%20Enum :default "NewEnumerator0") (skillDataREF :type Skill%20Data%20Structure%20Structure))
  (bind _refplayerequippedskills (Variables|Default|GetREFPlayerEquippedSkills))
  (LocalVariables|SetskillToEquip skillDataREF)
  (switch Utilities|FlowControl|Switch|SwitchonskillTypes skillByType
    (:NewEnumerator0
      (Utilities|Array|RemoveIndex _refplayerequippedskills)
      (Utilities|Array|Insert _refplayerequippedskills (LocalVariables|GetskillToEquip)))
    (:NewEnumerator1
      (Utilities|Array|RemoveIndex _refplayerequippedskills 1)
      (Utilities|Array|Insert _refplayerequippedskills (LocalVariables|GetskillToEquip) 1))
    (:NewEnumerator2
      (Utilities|Array|RemoveIndex _refplayerequippedskills 2)
      (Utilities|Array|Insert _refplayerequippedskills (LocalVariables|GetskillToEquip) 2))
    (:NewEnumerator3
      (Utilities|Array|RemoveIndex _refplayerequippedskills 3)
      (Utilities|Array|Insert _refplayerequippedskills (LocalVariables|GetskillToEquip) 3)))
  (return))

(fn AddSkilltoAllSkillsbySkillData
  (params (skillData :type Array%20of%20Skill%20Data%20Structure%20Structures))
  (for _array_element skillData
    (CallFunction|AddSkilltoAllSkillsbySkillName (Utilities|Array|MakeArray (Utilities|String|StringToName (.SkillName (Utilities|Struct|BreakSkillDataStructure _array_element))))))
  (return))

(fn GetSkillDatabyName
  (params (skillName :type Name))
  (bind _returnvalue (Utilities|GetDataTableRow "/Game/BlueprintsAndMaps/Blueprints/WeaponAndSkillsBPs/SkillDataTable.SkillDataTable" skillName)
    (:then
      (return _returnvalue))))

(fn CalcRechargeHealAmount
  (bind _refplayerequippedskills (Variables|Default|GetREFPlayerEquippedSkills))
  (bind _output (Utilities|Array|Get(acopy) _refplayerequippedskills 2))
  (bind _skillstatsstructure (Utilities|Struct|BreakSkillDataStructure _output))
  (bind (_mindamagepercent _maxdamagepercent _numhits _minrechargeflat _maxrechargeflat) (Utilities|Struct|BreakSkillStatsStructure _skillstatsstructure))
  (return (* (Math|Random|RandomIntegerinRange _minrechargeflat _maxrechargeflat) (Variables|Default|GetREFPlayerLevel))))

(fn ReturnSkillMaterialandIcononEnum
  (params (skillType :type skillTypes%20Enum :default "NewEnumerator0"))
  (bind _refplayerequippedskills (Variables|Default|GetREFPlayerEquippedSkills))
  (bind _refplayerequippedskills_2 (Variables|Default|GetREFPlayerEquippedSkills))
  (bind _refplayerequippedskills_3 (Variables|Default|GetREFPlayerEquippedSkills))
  (bind _refplayerequippedskills_4 (Variables|Default|GetREFPlayerEquippedSkills))
  (bind _output (Utilities|Array|Get(acopy) _refplayerequippedskills 3))
  (bind _output_2 (Utilities|Array|Get(acopy) _refplayerequippedskills_2))
  (bind _output_3 (Utilities|Array|Get(acopy) _refplayerequippedskills_3 1))
  (bind _output_4 (Utilities|Array|Get(acopy) _refplayerequippedskills_4 2))
  (bind (_skilltype _skillpassivearray _skillid _skillname _skillicon _skillstatsstructure _skillanimation _skillmaterial) (Utilities|Struct|BreakSkillDataStructure _output))
  (bind (_skilltype_2 _skillpassivearray_2 _skillid_2 _skillname_2 _skillicon_2 _skillstatsstructure_2 _skillanimation_2 _skillmaterial_2) (Utilities|Struct|BreakSkillDataStructure _output_2))
  (bind (_skilltype_3 _skillpassivearray_3 _skillid_3 _skillname_3 _skillicon_3 _skillstatsstructure_3 _skillanimation_3 _skillmaterial_3) (Utilities|Struct|BreakSkillDataStructure _output_3))
  (bind (_skilltype_4 _skillpassivearray_4 _skillid_4 _skillname_4 _skillicon_4 _skillstatsstructure_4 _skillanimation_4 _skillmaterial_4) (Utilities|Struct|BreakSkillDataStructure _output_4))
  (switch Utilities|FlowControl|Switch|SwitchonskillTypes skillType
    (:NewEnumerator0
      (LocalVariables|SetRETSkillIcon _skillicon_2)
      (LocalVariables|SetRETSkillMaterial _skillmaterial_2))
    (:NewEnumerator1
      (LocalVariables|SetRETSkillIcon _skillicon_3)
      (LocalVariables|SetRETSkillMaterial _skillmaterial_3))
    (:NewEnumerator2
      (LocalVariables|SetRETSkillIcon _skillicon_4)
      (LocalVariables|SetRETSkillMaterial _skillmaterial_4))
    (:NewEnumerator3
      (LocalVariables|SetRETSkillIcon _skillicon)
      (LocalVariables|SetRETSkillMaterial _skillmaterial))
    (:NewEnumerator4
      _))
  (return (LocalVariables|GetRETSkillIcon) (LocalVariables|GetRETSkillMaterial)))

(fn EquipItemtoSlot
  (params (weaponToEquip :type Weapon%20Data%20Structure%20Structure))
  (LocalVariables|SetweaponEquipping weaponToEquip)
  (for _array_element (Variables|Default|GetREFPlayerAllWeapons)
    (Utilities|Array|Add (LocalVariables|GetcurrentWeapons) _array_element))
  (bind _returnvalue (Utilities|Array|RemoveItem (LocalVariables|GetcurrentWeapons) (LocalVariables|GetweaponEquipping)))
  (if _returnvalue
    (Utilities|Array|Insert (LocalVariables|GetcurrentWeapons) (LocalVariables|GetweaponEquipping))
    (Variables|Default|SetREFPlayerAllWeapons (LocalVariables|GetcurrentWeapons))))

(fn GiveResourcetoPlayer
  (params (resourceName :type Name) (resourceAmount :type Integer) (resourceType :type resourceEnum%20Enum :default "NewEnumerator0"))
  (LocalVariables|SetresourceAmountToAdd resourceAmount)
  (LocalVariables|SetresourceNameToAdd resourceName)
  (LocalVariables|SetresourceTypeEnum resourceType)
  (bind (_array_element _array_index) (Utilities|Array|ForEachLoopwithBreak (Variables|Default|GetplayerOwnedResources) :!label _label)
    (:LoopBody
      (LocalVariables|SetresourceIndex _array_index)
      (LocalVariables|SetresourceOwned (Utilities|Name|Equal(Name) (.resourceName (Utilities|Struct|BreakresourceStruct _array_element)) (LocalVariables|GetresourceNameToAdd)))
      (if (Utilities|Name|Equal(Name) (.resourceName (Utilities|Struct|BreakresourceStruct _array_element)) (LocalVariables|GetresourceNameToAdd))
        (goto _label Break)))
    (:Completed
      (Utilities|Array|SetArrayElem (Variables|Default|GetplayerOwnedResources) (LocalVariables|GetresourceIndex) (Utilities|Struct|MakeresourceStruct (LocalVariables|GetresourceNameToAdd) (LocalVariables|GetresourceTypeEnum) (.resourceicon (Utilities|Array|Get(acopy) (Variables|Default|GetplayerOwnedResources) (LocalVariables|GetresourceIndex))) (+ (.resourceamount (Utilities|Array|Get(acopy) (Variables|Default|GetplayerOwnedResources) (LocalVariables|GetresourceIndex))) (LocalVariables|GetresourceAmountToAdd))) (not (LocalVariables|GetresourceOwned)))
      ;[1 1 1] Temp
      (for _array_element_2 (Variables|Default|GetplayerOwnedResources)
        (Development|PrintString 0 (Utilities|String|Append (Utilities|String|ToString(Name) (.resourceName (Utilities|Struct|BreakresourceStruct _array_element_2))) (Utilities|String|ToString(Integer) (.resourceAmount (Utilities|Struct|BreakresourceStruct _array_element_2))))))
      (return))))

(fn SetTotalPower
  (bind _refplayerlevel (Variables|Default|GetREFPlayerLevel))
  (bind _refplayerlevel_2 (Variables|Default|GetREFPlayerLevel))
  (bind _refbasepowerlevel (Variables|Default|GetREFBasePowerLevel))
  (bind _unitlvlpowermodifier (Variables|Default|GetunitLvlPowerModifier))
  (bind _refbasepowerlevel_2 (Variables|Default|GetREFBasePowerLevel))
  (bind _refbasepowerlevel_3 (Variables|Default|GetREFBasePowerLevel))
  (bind _currentweaponpower (Variables|Default|GetcurrentWeaponPower))
  (bind _currentweaponpower_2 (Variables|Default|GetcurrentWeaponPower))
  (bind _unitlvlpowermodifier_2 (Variables|Default|GetunitLvlPowerModifier))
  (bind _unitlvlpowermodifier_3 (Variables|Default|GetunitLvlPowerModifier))
  (bind _returnvalue (* _currentweaponpower_2 _unitlvlpowermodifier_3))
  (bind _returnvalue_2 (* _refbasepowerlevel_2 _unitlvlpowermodifier))
  (bind _returnvalue_3 (+ _refplayerlevel 1))
  (bind _returnvalue_4 (* _refbasepowerlevel _refplayerlevel_2))
  (bind _returnvalue_5 (Math|Conversions|ToFloat(Integer) _returnvalue_3))
  (bind _returnvalue_6 (Math|Conversions|ToFloat(Integer) _returnvalue_4))
  (bind _returnvalue_7 (Math|Float|Truncate _returnvalue))
  (bind _returnvalue_8 (Math|Float|Truncate _returnvalue_2))
  (bind _returnvalue_9 (Math|Float|Power _returnvalue_6 2.0))
  (bind _returnvalue_10 (* _returnvalue_5 _unitlvlpowermodifier_2))
  (bind _returnvalue_11 (+ _currentweaponpower _returnvalue_7))
  (bind _returnvalue_12 (+ _refbasepowerlevel_3 _returnvalue_8))
  (bind _returnvalue_13 (Math|Float|Log _returnvalue_10 2.0))
  (bind _returnvalue_14 (Math|Conversions|ToFloat(Integer) _returnvalue_12))
  (bind _returnvalue_15 (Math|Conversions|ToFloat(Integer) _returnvalue_11))
  (bind _returnvalue_16 (+ _returnvalue_14 _returnvalue_15))
  (bind _returnvalue_17 (+ _returnvalue_9 _returnvalue_16))
  (bind _returnvalue_18 (* _returnvalue_13 _returnvalue_17))
  (bind _returnvalue_19 (Math|Float|Truncate _returnvalue_18))
  (CallFunction|GetWeaponPower)
  (Variables|Default|SetREFTotalPowerLevel _returnvalue_19)
  (return _returnvalue_19))

(fn GetWeaponPower
  (Variables|Default|SetcurrentWeaponPower (.bonuspowerflat (Utilities|Array|Get(acopy) (.weaponpassivestructs (Utilities|Array|Get(acopy) (Variables|Default|GetREFPlayerAllWeapons))))))
  (return))

(fn CheckEnergy
  (params (skillType :type skillTypes%20Enum :default "NewEnumerator0"))
  (switch Utilities|FlowControl|Switch|SwitchonskillTypes skillType
    (:NewEnumerator0
      (if (>= (- (Variables|Default|GetREFPlayerCurrentEnergy) 0) 0)
        (Variables|Default|SetREFPlayerCurrentEnergy (- (Variables|Default|GetREFPlayerCurrentEnergy) 0))
        (LocalVariables|Setret (>= (- (Variables|Default|GetREFPlayerCurrentEnergy) 0) 0))))
    (:NewEnumerator1
      (if (>= (- (Variables|Default|GetREFPlayerCurrentEnergy) 4) 0)
        (Variables|Default|SetREFPlayerCurrentEnergy (- (Variables|Default|GetREFPlayerCurrentEnergy) 4))
        (LocalVariables|Setret (>= (- (Variables|Default|GetREFPlayerCurrentEnergy) 4) 0))))
    (:NewEnumerator2
      (if (>= (- (Variables|Default|GetREFPlayerCurrentEnergy) 2) 0)
        (Variables|Default|SetREFPlayerCurrentEnergy (- (Variables|Default|GetREFPlayerCurrentEnergy) 2))
        (LocalVariables|Setret (>= (- (Variables|Default|GetREFPlayerCurrentEnergy) 2) 0)))))
  (return (LocalVariables|Getret)))