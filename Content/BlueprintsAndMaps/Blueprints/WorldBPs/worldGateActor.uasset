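; World gate actor that moves the overworld player to another map when they walk into it.
; On overlap it stores the opposite compass direction of its own gate in the game instance as the spawn point, shows a travel screen, then opens the target level after a short random delay.
; activateSelf toggles the sprite's visibility and, when activated, replays a scaling timeline on it with a brief pause between runs.
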(event Custom|activateSelf
  (params (activate? :type Boolean))
  (Rendering|SetVisibility (Variables|Default|GetPaperSprite) activate? false)
  (if activate?
    (bind _newtrack_0 (Timeline|scaleSpriteTL PlayFromStart)
      (:Update
        (Transformation|SetRelativeScale3D (Variables|Default|GetPaperSprite) (Math|Vector|MakeVector _newtrack_0 _newtrack_0 _newtrack_0)))
      (:Finished
        (Utilities|FlowControl|Delay 0.2)
        (Timeline|scaleSpriteTL PlayFromStart)))))

(event EventBeginPlay)

(event Collision|EventActorBeginOverlap
  (params (OtherActor :type Actor%20Object%20Reference))
  (Utilities|Casting|CastTooverworldPlayerBP OtherActor)
  (bind _retspawngate (CallFunction|DetermineSpawnGate))
  (bind _asmain_game_instance (Utilities|Casting|CastTomainGameInstance (Game|GetGameInstance)))
  (Variables|/Game/BlueprintsAndMaps/Blueprints/GameBPs/mainGameInstance.mainGameInstance_C|SetplayerShouldSpawnHere _asmain_game_instance _retspawngate)
  (bind _returnvalue (UserInterface|CreateWidget "/Game/BlueprintsAndMaps/Blueprints/UI_BPs/TravelScreen.TravelScreen_C" (Game|GetPlayerController 0)))
  (UserInterface|Viewport|AddtoViewport _returnvalue 0)
  (Utilities|FlowControl|Delay (Math|Random|RandomFloatinRange 0.5 1.0))
  (Game|OpenLevel(byName) (Variables|Default|GetmapToTravelName)))

(event EventTick
  (params (DeltaSeconds :type Float%20%28single-precision%29)))

(fn ConstructionScript)

(fn DetermineSpawnGate
  (switch Utilities|FlowControl|Switch|SwitchongateEnums (Variables|Default|GetmyGateEnum)
    (:NewEnumerator0
      (LocalVariables|SetretEnum "NewEnumerator2"))
    (:NewEnumerator1
      (LocalVariables|SetretEnum "NewEnumerator3"))
    (:NewEnumerator2
      (LocalVariables|SetretEnum "NewEnumerator0"))
    (:NewEnumerator3
      (LocalVariables|SetretEnum "NewEnumerator1")))
  (return (LocalVariables|GetretEnum)))