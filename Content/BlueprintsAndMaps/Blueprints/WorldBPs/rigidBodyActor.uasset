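; A world obstacle actor that bounces the overworld player pawn off it on hit and can swap its material so players can see themselves behind it.
; On hit, if the pawn is not already bouncing, it mirrors the pawn's launch-time forward vector about the hit normal, turns the pawn that way and launches it.
; Horizontal launch strength scales with hit-to-pawn distance, with fixed upward velocity.
; A ReverseRotation yaw helper exists but is not called here.
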(event Custom|toggleVisibility
  (params (newVisibility :type Boolean))
  ;[1 1 1] Toggle Visible of these RIgidBodyActors so that players can see themselves behind them.
  (if newVisibility
    (Rendering|Material|SetMaterial (Variables|Default|GettestCube) 0 "/Engine/BasicShapes/BasicShapeMaterial.BasicShapeMaterial")
    (Variables|Default|SetisHidden false)
    (else
      (Rendering|Material|SetMaterial (Variables|Default|GettestCube) 0 "/Game/MyMaterials/BasicGreenMat1_2.BasicGreenMat1_2")
      (Variables|Default|SetisHidden true))))

(event Collision|EventHit
  (params (MyComp :type Primitive%20Component%20Object%20Reference) (Other :type Actor%20Object%20Reference) (OtherComp :type Primitive%20Component%20Object%20Reference) (bSelfMoved :type Boolean) (HitLocation :type Vector :default "0, 0, 0") (HitNormal :type Vector :default "0, 0, 0") (NormalImpulse :type Vector :default "0, 0, 0") (Hit :type Hit%20Result%20Structure%20%28by%20ref%29))
  ;[1 1 1] On Event Hit check if Player pawn hit, if so check if Player is NOT bouncing, if so set bounciness to default and set the flag on the PlayerBP Player Bounced.
  (bind _asoverworld_player_bp (Utilities|Casting|CastTooverworldPlayerBP Other))
  (bind _output_get (Variables|Default|SethitPlayerPawn _asoverworld_player_bp))
  (if (not (Variables|/Game/BlueprintsAndMaps/Blueprints/PlayerBPs/overworldPlayerBP.overworldPlayerBP_C|GetisBouncing _output_get))
    (Variables|Default|Setbounciness (Variables|Default|GetinitialBounciness))
    (Variables|/Game/BlueprintsAndMaps/Blueprints/PlayerBPs/overworldPlayerBP.overworldPlayerBP_C|SetplayerBounced (Variables|Default|GethitPlayerPawn) true)
    (Variables|/Game/BlueprintsAndMaps/Blueprints/PlayerBPs/overworldPlayerBP.overworldPlayerBP_C|SetisBouncing (Variables|Default|GethitPlayerPawn) true)
    (Variables|Default|Setbounciness (* (Math|Vector|VectorLength (- HitLocation (Transformation|GetActorLocation (Variables|Default|GethitPlayerPawn)))) 0.35))
    ;[1 1 1] Set Bounce Rotation and Velocity and Bounce.
    (bind _output_get_2 (Variables|/Game/BlueprintsAndMaps/Blueprints/PlayerBPs/overworldPlayerBP.overworldPlayerBP_C|SetbouncedRotation (Variables|Default|GethitPlayerPawn) (Math|Rotator|MakeRotator 0.0 0.0 (.yaw (Math|Conversions|RotationFromXVector (Math|Vector|MirrorVectorbyNormal (* (Math|Vector|GetForwardVector (Variables|/Game/BlueprintsAndMaps/Blueprints/PlayerBPs/overworldPlayerBP.overworldPlayerBP_C|GetcharacterRotAtLaunch (Variables|Default|GethitPlayerPawn))) (Math|Vector|VectorLength (- HitLocation (Transformation|GetActorLocation (Variables|Default|GethitPlayerPawn))))) HitNormal))))))
    (Transformation|SetActorRotation (Variables|Default|GethitPlayerPawn) _output_get_2 true)
    (Character|LaunchCharacter (Variables|Default|GethitPlayerPawn) (Math|Vector|MakeVector (.x (* (Math|Vector|MirrorVectorbyNormal (* (Math|Vector|GetForwardVector (Variables|/Game/BlueprintsAndMaps/Blueprints/PlayerBPs/overworldPlayerBP.overworldPlayerBP_C|GetcharacterRotAtLaunch (Variables|Default|GethitPlayerPawn))) (Math|Vector|VectorLength (- HitLocation (Transformation|GetActorLocation (Variables|Default|GethitPlayerPawn))))) HitNormal) (Variables|Default|Getbounciness))) (.y (* (Math|Vector|MirrorVectorbyNormal (* (Math|Vector|GetForwardVector (Variables|/Game/BlueprintsAndMaps/Blueprints/PlayerBPs/overworldPlayerBP.overworldPlayerBP_C|GetcharacterRotAtLaunch (Variables|Default|GethitPlayerPawn))) (Math|Vector|VectorLength (- HitLocation (Transformation|GetActorLocation (Variables|Default|GethitPlayerPawn))))) HitNormal) (Variables|Default|Getbounciness))) 2e+02) true true)))

(fn ConstructionScript)

(fn ReverseRotation
  (params (impactRot :type Rotator))
  (LocalVariables|SetrotYaw (.Yaw (Math|Rotator|BreakRotator impactRot)))
  (if (and (<= (LocalVariables|GetrotYaw) 0.0) (>= (LocalVariables|GetrotYaw) -179.0))
    (LocalVariables|SetrotYaw (* (LocalVariables|GetrotYaw) -1.0))
    (elif (and (>= (LocalVariables|GetrotYaw) 0.0) (< (LocalVariables|GetrotYaw) 9e+01))
      (LocalVariables|SetrotYaw (- 1.8e+02 (LocalVariables|GetrotYaw)))
      (elif (> (LocalVariables|GetrotYaw) 9e+01)
        (LocalVariables|SetrotYaw (- 1.8e+02 (LocalVariables|GetrotYaw))))))
  (return (Math|Rotator|MakeRotator 0.0 0.0 (LocalVariables|GetrotYaw))))